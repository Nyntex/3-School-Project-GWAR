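; Placeable spawner that spawns random actor classes in timed batches within a box, starting on BeginPlay or a one-time trigger.
; SpawnCycle places actors in range or on traced ground, retrying when the trace fails or finds nearby pawns or destructibles.
; CanStillSpawnMoreActors enforces a total or concurrent cap, with EndPlay callbacks freeing slots.
; ApplyOverrides replaces gem drop weights on spawned BP_EnemyBase actors.
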(event `self.ReceiveBeginPlay`
  (bind _basespawner (`self.BaseSpawner`))
  (bind _output_get (set `BaseSpawner.spawningEnabled` (`BaseSpawner.activeOnStart` _basespawner) _basespawner))
  (if _output_get
    (`KismetSystemLibrary.Delay` 1.0)
    (`self.Start Spawncycle`)))

(event `/Game/GeneralLogic/BPI_Triggerable.Trigger`
  (`/Engine/EditorBlueprintResources/StandardMacros.DoOnce` false
    (:`Completed`
      (bind _spawning (`BaseSpawner.Trigger` (`self.BaseSpawner`) false))
      (if _spawning
        (`self.Start Spawncycle`)))))

(event `SpawnCycle`
  (bind _basespawner (`self.BaseSpawner`))
  (if (<= (`self.Index`) (- (`BaseSpawner.amountToSpawn` (`self.BaseSpawner`)) 1))
    (`/Engine/EditorBlueprintResources/StandardMacros.IncrementInt` (`self.Index`)
      (:`  `
        (`KismetSystemLibrary.Delay` 0.02)
        (`self.CanStillSpawnMoreActors`
          (:`SpawnMore`
            (set `self.SpawnTries` 0)
            (if (`BaseSpawner.spawnOnGround` (`self.BaseSpawner`))
              (bind (_returnvalue _outhit) (`self.GetRandomPointOnGround` :!label _label))
              (if _returnvalue
                (bind (_bblockinghit _binitialoverlap _time _distance _location _impactpoint _normal _impactnormal _physmat _hitactor) (`GameplayStatics.BreakHitResult` _outhit))
                (cast `Pawn` _hitactor
                  (:`then`
                    ;[1 1 1] If "Ground" was another Pawn we retry the spawn 3 times
                    (if (< (`self.SpawnTries`) 3) :!label _label_2
                      (`/Engine/EditorBlueprintResources/StandardMacros.IncrementInt` (`self.SpawnTries`)
                        (:`  `
                          (goto _label)))
                      (else
                        (`KismetSystemLibrary.PrintString` "Actor Spawn Failed" :!label _label_3)
                        (`self.SpawnCycle`))))
                  (:`CastFailed`
                    (bind _returnvalue_2 (`|SpawnActorFromClass` (`BaseSpawner.GetRandomActorClass` (`self.BaseSpawner`)) (`KismetMathLibrary.MakeTransform` (+ _location (0.0 0.0 100.0)) (`KismetMathLibrary.MakeRotator` 0.0 0.0 (* (`KismetMathLibrary.RandomFloat`) 360.0))) "AdjustIfPossibleButDontSpawnIfColliding" "MultiplyWithRoot" null null))
                    (`/Engine/EditorBlueprintResources/StandardMacros.IsValid` _returnvalue_2
                      (:`Is Valid`
                        (add `self.OnEndPlay` _returnvalue_2 (delegate `SpawnedActorDied`))
                        (`KismetArrayLibrary.Array_Add` (`BaseSpawner.spawnedActors` (`self.BaseSpawner`)) _returnvalue_2)
                        (`self.ApplyOverrides` _returnvalue_2)
                        (bind _result (`/Engine/EditorBlueprintResources/StandardMacros.IncrementInt` (`self.currentlySpawned`))
                          (:`  `
                            (`KismetSystemLibrary.PrintString` (`KismetStringLibrary.Conv_IntToString` _result))
                            (`/Engine/EditorBlueprintResources/StandardMacros.IncrementInt` (`BaseSpawner.amountSpawned` (`self.BaseSpawner`)) :!label _label_4
                              (:`  `
                                (`self.SpawnCycle`))))))
                      (:`Is Not Valid`
                        (goto _label_3)))))
                (else
                  (goto _label_2)))
              (else
                (bind _returnvalue_3 (`|SpawnActorFromClass` (`BaseSpawner.GetRandomActorClass` _basespawner) (`KismetMathLibrary.MakeTransform` (`BaseSpawner.FindPositionInRange` _basespawner false) (`KismetMathLibrary.MakeRotator` 0.0 0.0 (* (`KismetMathLibrary.RandomFloat`) 360.0))) "AdjustIfPossibleButDontSpawnIfColliding" "MultiplyWithRoot" null null))
                (`/Engine/EditorBlueprintResources/StandardMacros.IsValid` _returnvalue_3
                  (:`Is Valid`
                    (add `self.OnEndPlay` _returnvalue_3 (delegate `SpawnedActorDied`))
                    (`KismetArrayLibrary.Array_Add` (`BaseSpawner.spawnedActors` (`self.BaseSpawner`)) _returnvalue_3)
                    (`self.ApplyOverrides` _returnvalue_3)
                    (goto _label_4))))))
          (:`StopSpawning`
            (`KismetSystemLibrary.Delay` (`BaseSpawner.timeBetweenSpawns` (`self.BaseSpawner`)) :!label _label_5)
            (set `self.Index` 0)
            (`self.Start Spawncycle`))
          (:`NextCycle`
            (goto _label_5)))))
    (else
      (goto _label_5))))

(event `Start Spawncycle`
  (if (`BaseSpawner.spawningEnabled` (`self.BaseSpawner`))
    (if (> (`KismetArrayLibrary.Array_Length` (`BaseSpawner.actorsToSpawn` (`self.BaseSpawner`))) 0)
      (`self.CanStillSpawnMoreActors`
        (:`SpawnMore`
          (`self.SpawnCycle`))
        (:`NextCycle`
          (goto _label_5))))))

(event `SpawnedActorDied` :!signature `self.OnEndPlay`
  (params (Actor :type "Actor Object Reference") (EndPlayReason :type "EEndPlayReason Enum" :default "Destroyed"))
  ;[0.2812 0.2812 0.2812] Check when an enemy dies so we can remove him from the array allowing us to spawn new units if max != total
  (`KismetArrayLibrary.Array_RemoveItem` (`BaseSpawner.spawnedActors` (`self.BaseSpawner`)) Actor)
  (`/Engine/EditorBlueprintResources/StandardMacros.DecrementInt` (`self.currentlySpawned`)))

(fn `ApplyOverrides`
  (params (Actor :type "Actor Object Reference"))
  (bind _nulldropweightoverwrite (`self.NullDropWeightOverwrite`))
  (bind _movementgemdropweightoverwrite (`self.MovementGemDropWeightOverwrite`))
  (bind _heavygemdropweightoverwrite (`self.HeavyGemDropWeightOverwrite`))
  (bind _fastgemdropweightoverwrite (`self.FastGemDropWeightOverwrite`))
  (bind _asbp_enemy_base (cast `/Game/Enemies/BaseLogic/BP_EnemyBase` Actor))
  (if (not (< _fastgemdropweightoverwrite 0))
    (set `/Game/Enemies/BaseLogic/BP_EnemyBase.FastGemDropWeight` _fastgemdropweightoverwrite _asbp_enemy_base))
  (if (not (< _heavygemdropweightoverwrite 0))
    (set `/Game/Enemies/BaseLogic/BP_EnemyBase.HeavyGemDropWeight` _heavygemdropweightoverwrite _asbp_enemy_base))
  (if (not (< _movementgemdropweightoverwrite 0))
    (set `/Game/Enemies/BaseLogic/BP_EnemyBase.MovementGemDropWeight` _movementgemdropweightoverwrite _asbp_enemy_base))
  (if (not (< _nulldropweightoverwrite 0))
    (set `/Game/Enemies/BaseLogic/BP_EnemyBase.NullDropWeight` _nulldropweightoverwrite _asbp_enemy_base)))

(fn `GetRandomPointOnGround`
  (returns (ReturnValue :type Boolean) (OutHit :type "HitResult Structure"))
  (locals (CheckDistanceExtender :type "Float (double-precision)" :default 500.0) (RandomPosition :type "Vector Structure"))
  (bind _basespawner (`self.BaseSpawner`))
  (bind (_returnvalue_x _returnvalue_y _returnvalue_z) (`KismetMathLibrary.BreakVector` (`BoxComponent.GetScaledBoxExtent` (`BaseSpawner.spawnBox` (`self.BaseSpawner`)))))
  (bind (_returnvalue_x_2 _returnvalue_y_2 _returnvalue_z_2) (`KismetMathLibrary.BreakVector` (`BoxComponent.GetScaledBoxExtent` (`BaseSpawner.spawnBox` _basespawner))))
  (bind _output_get (set `local.RandomPosition` (`BaseSpawner.FindPositionInRange` _basespawner false)))
  (bind (_outhit _returnvalue) (`KismetSystemLibrary.LineTraceSingle` :`Start` _output_get :`End` (+ _output_get (`KismetMathLibrary.MakeVector` 0.0 0.0 (- (* _returnvalue_z_2 -2.0) (`local.CheckDistanceExtender`)))) :`TraceChannel` "TraceTypeQuery2" :`DrawDebugType` "ForDuration" :`DrawTime` 0.5))
  (if _returnvalue
    (bind (_outactors _returnvalue_2) (`KismetSystemLibrary.SphereOverlapActors` (+ (`local.RandomPosition`) (`KismetMathLibrary.MakeVector` 0.0 0.0 (- (* _returnvalue_z -2.0) (`local.CheckDistanceExtender`)))) 200.0 (`|MakeArray` "ObjectTypeQuery3" "ObjectTypeQuery6" :!type "EObjectTypeQuery Enum")))
    (if _returnvalue_2
      (return false)
      (else
        (return _returnvalue _outhit)))
    (else
      (return false))))

(fn `UserConstructionScript`)
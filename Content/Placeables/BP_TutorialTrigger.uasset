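; BP_TutorialTrigger is a placeable one-shot trigger that shows a tutorial prompt when BP_PlayerCharacter overlaps it.
; It reads GamepadActive from BP_GameInstance to pick either the gamepad or the mouse-and-keyboard prompt widget class, held in its PromptToShowGamepad and PromptToShowMKB variables.
; The chosen widget is created for player 0 and added to the viewport, then the trigger destroys itself.
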(event `self.ReceiveActorBeginOverlap`
  (params (OtherActor :type "Actor Object Reference"))
  (bind _returnvalue (`GameplayStatics.GetPlayerController` 0))
  (cast `/Game/Player/Logic/BP_PlayerCharacter` OtherActor)
  (bind _asbp_game_instance (cast `/Game/GeneralLogic/BP_GameInstance` (`GameplayStatics.GetGameInstance`)))
  (if (`/Game/GeneralLogic/BP_GameInstance.GamepadActive` _asbp_game_instance)
    (bind _returnvalue_2 (`|CreateWidget` (`self.PromptToShow_Gamepad`) _returnvalue))
    (`UserWidget.AddToViewport` _returnvalue_2 0)
    (else
      (bind _returnvalue_3 (`|CreateWidget` (`self.PromptToShow_MKB`) _returnvalue))
      (`UserWidget.AddToViewport` _returnvalue_3 0)))
  (`self.K2_DestroyActor`))

(fn `UserConstructionScript`)
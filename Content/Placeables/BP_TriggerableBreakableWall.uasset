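; Placeable breakable wall that can only be shattered by damage while it is triggered.
; Trigger toggles the Triggered flag and destroys the Cube component, while the Breakable starts with physics simulation off.
; The first damage received while triggered destroys the Box, crumbles the Breakable's cluster, applies a radial impulse from the impact point and plays a sound, guarded by a DoOnce.
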(event `self.ReceiveBeginPlay`
  (`PrimitiveComponent.SetSimulatePhysics` (`self.Breakable`) false))

(event `/Game/GeneralLogic/BPI_Damageable.ApplyDamage`
  (params (DamageInfo :type "/Game/GeneralLogic/S_DamageInfo Structure") (DamageCauser :type "Actor Object Reference"))
  (bind _breakable (`self.Breakable`))
  (if (`self.Triggered`)
    (`/Engine/EditorBlueprintResources/StandardMacros.DoOnce` false
      (:`Completed`
        (`ActorComponent.K2_DestroyComponent` (`self.Box`))
        (`GeometryCollectionComponent.CrumbleCluster` _breakable 0)
        (`PrimitiveComponent.AddRadialImpulse` _breakable DamageInfo_ImpactLocation_15_EFB68C5C4D6466E77A8C0587CD39F6FF 400.0 400.0 "RIF_Constant" true)
        (`GameplayStatics.PlaySoundAtLocation` null (`self.K2_GetActorLocation`) (struct) 1.0 1.0 0.0 null null null null)))))

(event `/Game/GeneralLogic/BPI_Triggerable.Trigger`
  (set `self.Triggered` (not (`self.Triggered`)))
  (`ActorComponent.K2_DestroyComponent` (`self.Cube`)))

(fn `GetWorldPosition`
  (returns (RetVal :type "Vector Structure"))
  (return (`self.K2_GetActorLocation`)))

(fn `UserConstructionScript`)
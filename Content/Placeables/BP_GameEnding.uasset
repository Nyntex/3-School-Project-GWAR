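; BP_GameEnding is a placeable trigger that ends the game when the player enters its box.
; On overlap by BP_PlayerCharacter it shows the WBP_CreditsOverlay widget, plays the referenced level sequence, removes the player's HUD and destroys the character.
; After a delay equal to the sequence's duration it opens MainMenuMap.
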(event `self.Box.OnComponentBeginOverlap`
  (params (OverlappedComponent :type "PrimitiveComponent Object Reference") (OtherActor :type "Actor Object Reference") (OtherComp :type "PrimitiveComponent Object Reference") (OtherBodyIndex :type Integer) (bFromSweep :type Boolean) (SweepResult :type "HitResult Structure (by ref)"))
  (bind _sequenceplayer (`LevelSequenceActor.SequencePlayer` (`self.SequenceRef`)))
  (bind _asbp_player_character (cast `/Game/Player/Logic/BP_PlayerCharacter` OtherActor))
  (bind _returnvalue (`|CreateWidget` "/Game/UI/OtherWidgets/WBP_CreditsOverlay.WBP_CreditsOverlay_C"))
  (`UserWidget.AddToViewport` _returnvalue 0)
  (`MovieSceneSequencePlayer.Play` _sequenceplayer)
  (`Widget.RemoveFromParent` (`/Game/Player/Logic/BP_PlayerCharacter.HUD` _asbp_player_character))
  (`self.K2_DestroyActor` _asbp_player_character)
  (`KismetSystemLibrary.Delay` (`TimeManagementBlueprintLibrary.Conv_QualifiedFrameTimeToSeconds` (`MovieSceneSequencePlayer.GetDuration` _sequenceplayer)))
  (`GameplayStatics.OpenLevel` "MainMenuMap"))

(fn `UserConstructionScript`)
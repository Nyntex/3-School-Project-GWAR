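; BP_DeathZone is a placeable kill volume that deals massive damage to actors that begin overlapping its Trigger component.
; With CanKillEnemies on, it damages any actor through BPI_Damageable, falling back to engine ApplyDamage for actors without that interface.
; With it off, only BP_PlayerCharacter takes damage.
; SetActive is an empty stub, so it does not toggle the zone.
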(event `self.Trigger.OnComponentBeginOverlap`
  (params (OverlappedComponent :type "PrimitiveComponent Object Reference") (OtherActor :type "Actor Object Reference") (OtherComp :type "PrimitiveComponent Object Reference") (OtherBodyIndex :type Integer) (bFromSweep :type Boolean) (SweepResult :type "HitResult Structure (by ref)"))
  (if (`self.CanKillEnemies`)
    (bind _asbpi_damageable (cast `/Game/GeneralLogic/BPI_Damageable` OtherActor)
      (:`then`
        (`/Game/GeneralLogic/BPI_Damageable.ApplyDamage` _asbpi_damageable (make `/Game/GeneralLogic/S_DamageInfo` "NewEnumerator0" 1000000.0) self))
      (:`CastFailed`
        (`GameplayStatics.ApplyDamage` OtherActor 1000.0)))
    (else
      (bind _asbp_player_character (cast `/Game/Player/Logic/BP_PlayerCharacter` OtherActor))
      (`/Game/GeneralLogic/BPI_Damageable.ApplyDamage` _asbp_player_character (make `/Game/GeneralLogic/S_DamageInfo` "NewEnumerator0" 1000.0) null))))

(fn `SetActive`
  (params (Active :type Boolean))
  (if Active
    _))

(fn `UserConstructionScript`)
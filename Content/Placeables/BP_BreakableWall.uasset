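; BP_BreakableWall is a placeable wall that breaks apart when it takes damage.
; Its geometry collection starts with physics simulation off; the first ApplyDamage event removes the Box component, crumbles the cluster and applies a radial impulse at the impact location.
; It plays a rock crumble sound and destroys the actor after a short delay, with a DoOnce preventing repeat triggers.
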(event `self.ReceiveBeginPlay`
  (`PrimitiveComponent.SetSimulatePhysics` (`self.GEOCOL_BreakableWall`) false))

(event `self.ReceiveActorBeginOverlap`
  (params (OtherActor :type "Actor Object Reference")))

(event `/Game/GeneralLogic/BPI_Damageable.ApplyDamage`
  (params (DamageInfo :type "/Game/GeneralLogic/S_DamageInfo Structure") (DamageCauser :type "Actor Object Reference"))
  (bind _geocol_breakablewall (`self.GEOCOL_BreakableWall`))
  (`/Engine/EditorBlueprintResources/StandardMacros.DoOnce` false
    (:`Completed`
      (`ActorComponent.K2_DestroyComponent` (`self.Box`))
      (`GeometryCollectionComponent.CrumbleCluster` _geocol_breakablewall 0)
      (`PrimitiveComponent.AddRadialImpulse` _geocol_breakablewall DamageInfo_ImpactLocation_15_EFB68C5C4D6466E77A8C0587CD39F6FF 400.0 400.0 "RIF_Constant" true)
      (`GameplayStatics.PlaySoundAtLocation` "/Game/Audio/SFX/MetaSounds/MS_RockCrumble.MS_RockCrumble" (`self.K2_GetActorLocation`) (struct) 1.0 1.0 0.0 null null null null)
      (`KismetSystemLibrary.Delay` 5.0)
      (`self.K2_DestroyActor`))))

(fn `GetWorldPosition`
  (returns (RetVal :type "Vector Structure"))
  (return (`self.K2_GetActorLocation`)))

(fn `UserConstructionScript`)
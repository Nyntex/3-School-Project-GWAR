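; Combat arena trigger that starts battle music and a blood meter when the player enters, then completes at a kill quota.
; Counts deaths of enemies inside or entering; destroyed spawners can credit their unspawned units.
; Completion breaks or destroys linked actors, fires triggerables and removes the arena.
; A construction-script ID optionally saves completion in the game instance, so finished arenas silently force-complete on BeginPlay.
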(event Custom|Enemy%20Died
  (params (Actor :type Actor%20Object%20Reference))
  (bind _bloodmeter (Variables|Default|GetBloodMeter))
  (bind _asbp_enemy_base (Utilities|Casting|CastToBP_EnemyBase Actor))
  (EventDispatchers|UnbindEventfromDie _asbp_enemy_base (EventDispatchers|CreateEvent :!event Custom|Enemy%20Died))
  (bind _result (Math|Integer|IncrementInt (Variables|Default|GetEnemiesKilled))
    (:%20%20
      (Variables|/Game/UI/HUD/WBP_BloodMeter.WBP_BloodMeter_C|SetEnemiesKilled _bloodmeter _result)
      (Default|ReloadBar _bloodmeter)
      (Utilities|EnemiestoKillReached
        (:True
          (CallFunction|AllEnemiesKilled false))))))

(event Custom|Spawner%20Destroyed
  (params (Actor :type Actor%20Object%20Reference) (EndPlayReason :type EEndPlayReason%20Enum :default "Destroyed"))
  (bind _bloodmeter (Variables|Default|GetBloodMeter))
  (bind _asbp_spawner_destructible (Utilities|Casting|CastToBP_Spawner_Destructible Actor))
  (Game|UnbindEventfromOnEndPlay (EventDispatchers|CreateEvent :!event Custom|Spawner%20Destroyed))
  (switch Utilities|FlowControl|Switch|SwitchonEEndPlayReason EndPlayReason
    (:Destroyed
      (bind _basespawner (Variables|/Game/Placeables/BP_BaseSpawner.BP_BaseSpawner_C|GetBaseSpawner _asbp_spawner_destructible)
        (:then
          (if (Variables|/Script/P3T3_Project.BaseSpawner|GetmaxUnitsIsTotal _basespawner)
            (bind _output_get (Variables|Default|SetEnemiesKilled (|(A+(B-C)) (Variables|Default|GetEnemiesKilled) (Variables|/Script/P3T3_Project.BaseSpawner|GetmaxUnitsToSpawn _basespawner) (Variables|/Script/P3T3_Project.BaseSpawner|GetamountSpawned _basespawner)) :!label _label))
            (Variables|/Game/UI/HUD/WBP_BloodMeter.WBP_BloodMeter_C|SetEnemiesKilled _bloodmeter _output_get)
            (Default|ReloadBar _bloodmeter)
            (Utilities|EnemiestoKillReached
              (:True
                (CallFunction|AllEnemiesKilled false)))
            (elif (< (Variables|/Script/P3T3_Project.BaseSpawner|GetamountSpawned _basespawner) (Variables|/Script/P3T3_Project.BaseSpawner|GetmaxUnitsToSpawn _basespawner))
              (goto _label))))
        (:else)))))

(event EventBeginPlay
  (bind _self self)
  (bind _returnvalue (Utilities|GetDisplayName _self))
  (if (<= (Variables|Default|GetEnemiesToKill) 0)
    (CallFunction|AllEnemiesKilled false)
    (Development|PrintString (Utilities|String|Append "ARENA HAS ENEMIES TO KILL SET TO 0: " _returnvalue))
    (elif (Variables|Default|GetSaveFinishedState)
      (Utilities|FlowControl|Delay 0.1)
      (bind _asbp_game_instance (Utilities|Casting|CastToBP_GameInstance (Game|GetGameInstance)))
      (if (>= (Utilities|Array|FindItem (Variables|/Game/GeneralLogic/BP_GameInstance.BP_GameInstance_C|GetFinishedArenasIDs _asbp_game_instance) (Variables|Default|GetID)) 0)
        (Development|PrintString (Utilities|String|Append "Arena already completed: " _returnvalue) true true "(R=0.000000,G=0.660000,B=1.000000,A=1.000000)" 5.0)
        (CallFunction|AllEnemiesKilled true)))))

(event Collision|EventActorBeginOverlap
  (params (OtherActor :type Actor%20Object%20Reference))
  (Variables|Default|GetBloodMeter
    (:then
      (|BindToEnemyDied OtherActor))
    (:else
      (Utilities|FlowControl|DoOnce false :!label _label
        (:Completed
          (bind _asbp_player_character (Utilities|Casting|CastToBP_PlayerCharacter OtherActor)
            (:then
              (CallFunction|SetupBloodMeterWidget _asbp_player_character)
              (bind _returnvalue (Audio|SpawnSound2D "/Game/Audio/Music/MS_CombatMusic.MS_CombatMusic" 1.0 1.0 0.0 0))
              (bind _output_get (Variables|Default|SetBattleMusic _returnvalue))
              (Audio|Components|Audio|FadeIn _output_get 3.0 1.0 0.0 "Linear" :!class /Script/Engine.AudioComponent)
              (for _array_element (Collision|GetOverlappingActors (Variables|Default|GetCollider) "/Script/P3T3_Project.EnemyBase" :!class /Script/Engine.PrimitiveComponent)
                (|BindToEnemyDied_2 _array_element))
              (for _array_element_2 (Collision|GetOverlappingActors (Variables|Default|GetCollider) "/Game/Placeables/BP_Spawner_Destructible.BP_Spawner_Destructible_C" :!class /Script/Engine.PrimitiveComponent)
                (|BindToSpawnerEndPlay _array_element_2)))
            (:CastFailed
              (goto _label Reset))))))))

(event EventTick
  (params (DeltaSeconds :type Float%20%28single-precision%29)))

(fn ConstructionScript
  (CallFunction|ValidateSetID))

(fn AllEnemiesKilled
  (params (Forced :type Boolean))
  (Development|PrintString (Utilities|String|Append "Arena completed: " (Utilities|GetDisplayName self) " 
Forced? : " (Utilities|String|ToString(Boolean) Forced)))
  (Utilities|FlowControl|Sequence
    (:then_0
      (for _array_element (Variables|Default|GetActorsToDestroyOnCompletion)
        (Utilities|IsValid _array_element
          (:Is%20Valid
            (if Forced
              (Actor|DestroyActor _array_element :!label _label)
              (else
                (bind _asbp_breakable_wall (Utilities|Casting|CastToBP_BreakableWall _array_element)
                  (:then
                    (Default|ApplyDamage _asbp_breakable_wall (Utilities|Struct|MakeS_DamageInfo "NewEnumerator0" 0.0 0.0 0.0 0.0 (Transformation|GetActorLocation)) self))
                  (:CastFailed
                    (goto _label)))))))))
    (:then_1
      (for _array_element_2 (Variables|Default|GetTriggerablesToTriggerOnCompletion)
        (bind _asbpi_triggerable (Utilities|Casting|CastToBPI_Triggerable _array_element_2))
        (Default|Trigger _asbpi_triggerable)))
    (:then_2
      (bind _bloodmeter (Variables|Default|GetBloodMeter)
        (:then
          (Widget|RemovefromParent _bloodmeter))
        (:else
          _))
      (if (Variables|Default|GetSaveFinishedState)
        (bind _asbp_game_instance (Utilities|Casting|CastToBP_GameInstance (Game|GetGameInstance)))
        (Utilities|Array|AddUnique (Variables|/Game/GeneralLogic/BP_GameInstance.BP_GameInstance_C|GetFinishedArenasIDs _asbp_game_instance) (Variables|Default|GetID))))
    (:then_3
      (if Forced
        _
        (else
          (Audio|PlaySoundatLocation "/Game/Audio/SFX/MetaSounds/MS_ClearedCombatZone.MS_ClearedCombatZone" (Transformation|GetActorLocation) "0, 0, 0" 1.0 1.0 0.0 0 0 0 0)
          (bind _battlemusic (Variables|Default|GetBattleMusic)
            (:then
              (Audio|Components|Audio|FadeOut _battlemusic 3.0 0.0 "Linear" :!class /Script/Engine.AudioComponent))
            (:else
              _))))
      (Actor|DestroyActor))
    (:then_4
      (Default|CallArenaCompleted Forced))))

(fn SetupBloodMeterWidget
  (params (OwningPlayer :type Pawn%20Object%20Reference))
  (bind _asplayer_controller (Utilities|Casting|CastToPlayerController (Pawn|GetController OwningPlayer)))
  (bind _returnvalue (UserInterface|CreateWidget (Variables|Default|GetBloodMeterWidgetClass) _asplayer_controller))
  (Development|PrintString "Hello")
  (bind _aswbp_blood_meter (Utilities|Casting|CastToWBP_BloodMeter _returnvalue))
  (bind _output_get (Variables|Default|SetBloodMeter _aswbp_blood_meter))
  (Variables|/Game/UI/HUD/WBP_BloodMeter.WBP_BloodMeter_C|SetEnemiesToKill _output_get (Variables|Default|GetEnemiesToKill))
  (Default|ReloadBar _output_get)
  (UserInterface|Viewport|AddtoViewport (Variables|Default|GetBloodMeter) 0))

(fn GenerateNewID
  (bind _idvalues (LocalVariables|GetIDValues))
  (for _index (range 0 (- (LocalVariables|GetIDSize) 1))
    (LocalVariables|SettempString (Utilities|String|Append (LocalVariables|GettempString) (Utilities|Array|Get(acopy) (Utilities|String|GetCharacterArrayfromString _idvalues) (Math|Random|RandomInteger (Utilities|String|Len _idvalues))))))
  (return (Utilities|String|StringToName (LocalVariables|GettempString))))

(fn ValidateSetID
  (if (== (Variables|Default|GetID) "")
    (bind _new_id (CallFunction|GenerateNewID))
    (Variables|Default|SetID _new_id)
    (else
      (bind _outactors (Actor|GetAllActorsOfClass "BP_Arena_C"))
      (bind _array_element (Utilities|Array|ForEachLoopwithBreak _outactors :!label _label)
        (:LoopBody
          (if (not (== _array_element self))
            (if (== (Variables|BP_Arena_C|GetID _array_element) (Variables|Default|GetID))
              (bind _new_id_2 (CallFunction|GenerateNewID))
              (Variables|Default|SetID _new_id_2)
              (goto _label Break))))
        (:Completed
          (if (== (Variables|Default|GetID) "")
            (bind _new_id_3 (CallFunction|GenerateNewID))
            (Variables|Default|SetID _new_id_3)))))))
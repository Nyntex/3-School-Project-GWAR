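; Destructible enemy spawner placeable that players can damage and destroy to shut off its spawning.
; Only damage from the player character counts, reducing health and playing an egg splat sound plus a damage-type-specific Niagara hit effect at the weapon's socket.
; When health runs out, it disables spawning on its base spawner component and destroys itself.
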(event `self.ReceiveBeginPlay`
  (`parent.ReceiveBeginPlay`)
  (set `self.currentHealth` (`self.MaxHealth`)))

(event `/Game/GeneralLogic/BPI_Damageable.ApplyDamage`
  (params (DamageInfo :type "/Game/GeneralLogic/S_DamageInfo Structure") (DamageCauser :type "Actor Object Reference"))
  (bind (_damagetype _damageamount) (break `/Game/GeneralLogic/S_DamageInfo` DamageInfo))
  (bind _asbp_player_character (cast `/Game/Player/Logic/BP_PlayerCharacter` DamageCauser))
  (bind _output_get (set `self.currentHealth` (- (`self.currentHealth`) _damageamount)))
  (`GameplayStatics.PlaySoundAtLocation` "/Game/Audio/SFX/MetaSounds/MS_EggSplat.MS_EggSplat" (`self.K2_GetActorLocation`) (struct) 1.0 1.0 0.0 null null null null)
  (`NiagaraFunctionLibrary.SpawnSystemAtLocation` (select `/Game/GeneralLogic/E_DamageType` _damagetype :`NewEnumerator0` "/Game/Enemies/VFX/Hit_FX/NS_Enemy_Hit_Neutral.NS_Enemy_Hit_Neutral" :`NewEnumerator1` "/Game/Enemies/VFX/Hit_FX/NS_Enemy_Hit_Lightning.NS_Enemy_Hit_Lightning" :`NewEnumerator2` "/Game/Enemies/VFX/Hit_FX/NS_Enemy_Hit_Poison.NS_Enemy_Hit_Poison" :`NewEnumerator4` "/Game/Enemies/VFX/Hit_FX/NS_Enemy_Hit_Neutral.NS_Enemy_Hit_Neutral" :`NewEnumerator5` "/Game/Enemies/VFX/Hit_FX/NS_Enemy_Hit_Neutral.NS_Enemy_Hit_Neutral" :!type "NiagaraSystem Object Reference") (`SceneComponent.GetSocketLocation` (`/Game/Player/Logic/BP_PlayerCharacter.Weapon` _asbp_player_character) "BottomSocket"))
  (if (<= _output_get 0.0)
    (set `BaseSpawner.spawningEnabled` false (`self.BaseSpawner`))
    (`self.K2_DestroyActor`)))

(fn `GetWorldPosition`
  (returns (RetVal :type "Vector Structure"))
  (return (`self.K2_GetActorLocation`)))

(fn `UserConstructionScript`
  (`parent.UserConstructionScript`))
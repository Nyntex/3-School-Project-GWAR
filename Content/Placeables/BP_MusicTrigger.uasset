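; BP_MusicTrigger is a placeable actor that plays a music Track in response to the player pawn overlapping it.
; The first overlap by player 0's pawn fades the Track in through a DoOnce that is never reset, so later entries do not restart it.
; Each exit by that pawn fades the Track out and schedules a delayed stop matching the fade length.
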(event `self.ReceiveActorBeginOverlap`
  (params (OtherActor :type "Actor Object Reference"))
  (if (== OtherActor (`GameplayStatics.GetPlayerPawn` 0))
    (`/Engine/EditorBlueprintResources/StandardMacros.DoOnce` false
      (:`Completed`
        (`AudioComponent.FadeIn` (`self.Track`) 1.0 1.0 0.0 "Linear")))))

(event `self.ReceiveActorEndOverlap`
  (params (OtherActor :type "Actor Object Reference"))
  (bind _track (`self.Track`))
  (if (== (`GameplayStatics.GetPlayerPawn` 0) OtherActor)
    (`AudioComponent.FadeOut` _track 1.0 0.0 "Linear")
    (`AudioComponent.StopDelayed` _track 1.0)))

(fn `UserConstructionScript`)
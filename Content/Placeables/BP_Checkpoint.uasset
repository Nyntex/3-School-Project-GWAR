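; Placeable checkpoint that, on first player overlap, becomes the current checkpoint and heals a percentage of max health.
; It records its ID in the game instance and checks that list on BeginPlay so it stays triggered.
; The construction script applies box size and positions the respawn arrow with wrapped yaw.
; It also generates a random ID when the ID is empty or duplicates another checkpoint's.
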(event `self.ReceiveBeginPlay`
  (bind _asbp_game_instance (cast `/Game/GeneralLogic/BP_GameInstance` (`GameplayStatics.GetGameInstance`)))
  (if (>= (`KismetArrayLibrary.Array_Find` (`/Game/GeneralLogic/BP_GameInstance.TriggeredCheckpoints` _asbp_game_instance) (`self.ID`)) 0)
    (set `self.AlreadyTriggered` true)))

(event `self.Box.OnComponentBeginOverlap`
  (params (OverlappedComponent :type "PrimitiveComponent Object Reference") (OtherActor :type "Actor Object Reference") (OtherComp :type "PrimitiveComponent Object Reference") (OtherBodyIndex :type Integer) (bFromSweep :type Boolean) (SweepResult :type "HitResult Structure (by ref)"))
  (if (not (`self.AlreadyTriggered`))
    (bind _asbp_player_character (cast `/Game/Player/Logic/BP_PlayerCharacter` OtherActor))
    (bind _asbp_game_instance (cast `/Game/GeneralLogic/BP_GameInstance` (`GameplayStatics.GetGameInstance`)))
    (bind _output_get (set `/Game/GeneralLogic/BP_GameInstance.CurrentCheckpointID` (`self.ID`) _asbp_game_instance))
    (`KismetArrayLibrary.Array_AddUnique` (`/Game/GeneralLogic/BP_GameInstance.TriggeredCheckpoints` _asbp_game_instance) _output_get)
    (set `self.AlreadyTriggered` true)
    (bind _bpc_playerstats (`/Game/Player/Logic/BP_PlayerCharacter.BPC_PlayerStats` _asbp_player_character))
    (`/Game/Player/Logic/BPC_PlayerStats.AddHealth` _bpc_playerstats (* (`/Game/Player/Logic/BPC_PlayerStats.MaxHealth` _bpc_playerstats) (`self.PercentHeal`)))))

(fn `CreateNewID`
  (locals (IDSize :type Integer :default 16) (IDValues :type String :default "ABCDEFGHIJKLMONPQRSTUVWXYZabcdefghijklmnopqrstuvwxyz0123456789") (tempString :type String))
  (bind _idvalues (`local.IDValues`))
  (for _ (range (`local.IDSize`))
    (set `local.tempString` (`KismetStringLibrary.Concat_StrStr` (`local.tempString`) (`|GetArrayItem` (`KismetStringLibrary.GetCharacterArrayFromString` _idvalues) (`KismetMathLibrary.RandomInteger` (`KismetStringLibrary.Len` _idvalues))))))
  (set `self.ID` (`KismetStringLibrary.Conv_StringToName` (`local.tempString`))))

(fn `UserConstructionScript`
  (`|ExecutionSequence`
    (:`then_0`
      (`BoxComponent.SetBoxExtent` (`self.Box`) (`self.BoxSize`) true)
      (`self.SetActorScale3D` (1.0 1.0 1.0))
      (`SceneComponent.K2_SetRelativeLocation` (`self.Arrow`) (`self.RespawnPosition`) false true)
      (if (< (`self.RespawnRotationYaw`) -180.0)
        (set `self.RespawnRotationYaw` (+ (`self.RespawnRotationYaw`) 360.0))
        (elif (> (`self.RespawnRotationYaw`) 180.0)
          (set `self.RespawnRotationYaw` (- (`self.RespawnRotationYaw`) 360.0))))
      (`SceneComponent.K2_SetWorldRotation` (`self.Arrow`) (`KismetMathLibrary.MakeRotator` 0.0 0.0 (`self.RespawnRotationYaw`)) false true))
    (:`then_1`
      ;[1 1 1] New ID
      (if (== (`self.ID`) "None")
        (`self.CreateNewID`)
        (else
          (bind _outactors (`GameplayStatics.GetAllActorsOfClass` "BP_Checkpoint_C"))
          (for _array_element _outactors
            (if (== _array_element self)
              _
              (elif (== (`/Game/Placeables/BP_Checkpoint.ID` _array_element) (`self.ID`))
                (`self.CreateNewID`)
                (break))))
          (if (== (`self.ID`) "None")
            (`self.CreateNewID`)))))))
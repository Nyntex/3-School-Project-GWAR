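; Flying Vomiter enemy that lobs projectiles at targets in range, using a custom-arc launch velocity with random spread.
; A stat component supplies its tuning, and chase, idle and state events drive FlyingMovement to approach, wander or stop, while fleeing uses movement input.
; Hits apply knockback, effects, lightning stun or poison damage over time, and death destroys the actor immediately.
; The montage-and-dissolve death and an older shooting loop are disconnected.
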(event `self.ReceiveBeginPlay`
  (bind _charactermovement (`self.CharacterMovement`))
  (`self.SetValuesFromStatComponent`)
  (bind _output_get (set `CharacterMovementComponent.MaxWalkSpeed` (`self.movementSpeed`) _charactermovement))
  (set `CharacterMovementComponent.MaxFlySpeed` _output_get _charactermovement)
  (`KismetSystemLibrary.Delay` 0.2)
  (bind _returnvalue (`PrimitiveComponent.CreateDynamicMaterialInstance` (`self.Mesh`) 0 "/Game/Enemies/Chaser/Effects/MI_EnemyDeath_Lightning_Inst.MI_EnemyDeath_Lightning_Inst" "None"))
  (bind _output_get_2 (set `self.DynamicMaterial` _returnvalue))
  (`MaterialInstanceDynamic.SetScalarParameterValue` _output_get_2 "Dissolve" 0.5))

(event `TryAttacking`
  (params (AttackTarget :type "Actor Object Reference"))
  (bind (_returnvalue_location _returnvalue_rotation _returnvalue_scale) (`KismetMathLibrary.BreakTransform` (`self.GetTransform`)))
  (if (`.inRange` (`self.IsActorInAttackRange` AttackTarget))
    ;[1 1 1 0.257 14] Attack
    (`/Engine/EditorBlueprintResources/StandardMacros.DoOnce` false :!label _label
      (:`Completed`
        (bind _returnvalue (`|SpawnActorFromClass` (`self.ObjectToShoot`) (`KismetMathLibrary.MakeTransform` (+ _returnvalue_location (`self.ShootPosition`)) _returnvalue_rotation _returnvalue_scale) "AlwaysSpawn" "MultiplyWithRoot" null null))
        (`/Engine/EditorBlueprintResources/StandardMacros.IsValid` _returnvalue
          (:`Is Valid`
            (bind _launch_velocity (`self.SuggestLaunchVelocity` AttackTarget))
            (`PrimitiveComponent.AddImpulse` (`self.GetComponentByClass` _returnvalue "/Script/Engine.StaticMeshComponent") _launch_velocity "None" true))
          (:`Is Not Valid`
            _))
        (`KismetSystemLibrary.Delay` (/ 1.0 (`self.attacksPerSecond`)))
        (`|ExecutionSequence`
          (:`then_0`
            (goto _label :!via `Reset`))
          (:`then_1`
            (`self.FinishedAttacking`)))))))

(event `Event ChangeState`
  (params (State :type "EEnemyStates Enum" :default "Invalid"))
  (bind _state (`self.ChangeState` State))
  (switch `EEnemyStates` _state
    (:`Invalid`
      (`/Game/Enemies/BaseLogic/BP_FlyingMovement_Component.StopMovement` (`self.Flying Movement`) true))
    (:`IDLE`
      (`/Game/Enemies/BaseLogic/BP_FlyingMovement_Component.StopMovement` (`self.Flying Movement`) false :!label _label_2))
    (:`FLEE`
      (goto _label_2))
    (:`CHASE`
      (goto _label_2))))

(event `Move_Chase`
  (if (`.inRange` (`self.IsActorInAttackRange` (`/Game/Enemies/BaseLogic/AIC_EnemyBase.TargetActor` (cast `/Game/Enemies/VomiterFlying/Logic/AIC_EnemyVomiter_Flying` (`self.GetController`) :!pure true))))
    (`/Game/Enemies/BaseLogic/BP_FlyingMovement_Component.StopMovement` (`self.Flying Movement`) true)
    (else
      (`/Engine/EditorBlueprintResources/StandardMacros.DoOnce` false :!label _label_3
        (:`Completed`
          (bind _asaic_enemy_base (cast `/Game/Enemies/BaseLogic/AIC_EnemyBase` (`self.GetController`)))
          (if (`/Game/Enemies/BaseLogic/BP_FlyingMovement_Component.DirectPathToTarget` (`self.Flying Movement`))
            (bind _targetactor (`/Game/Enemies/BaseLogic/AIC_EnemyBase.TargetActor` _asaic_enemy_base))
            (`/Game/Enemies/BaseLogic/BP_FlyingMovement_Component.MoveToNewPosition` (`self.Flying Movement`) (`self.GetAttackablePosition` _targetactor))
            (else
              (`/Game/Enemies/BaseLogic/BP_FlyingMovement_Component.MoveToActor` (`self.Flying Movement`) _targetactor)))
          (`KismetSystemLibrary.Delay` 0.2)
          (goto _label_3 :!via `Reset`))))))

(event `Move_Idle`
  (if (`/Game/Enemies/BaseLogic/BP_FlyingMovement_Component.FinishedMovment` (`self.Flying Movement`))
    (`/Game/Enemies/BaseLogic/BP_FlyingMovement_Component.MoveToRandomPosition` (`self.Flying Movement`))))

(event `Move_Flee`
  (params (FleeTarget :type "Actor Object Reference"))
  (bind (_returnvalue_x _returnvalue_y) (`KismetMathLibrary.BreakVector` (- (`self.K2_GetActorLocation`) (`self.K2_GetActorLocation` FleeTarget))))
  (`/Engine/EditorBlueprintResources/StandardMacros.IsValid` FleeTarget
    (:`Is Valid`
      (`self.AddMovementInput` (`KismetMathLibrary.Normal` (`KismetMathLibrary.MakeVector` _returnvalue_x _returnvalue_y))))))

(event `self.Flying Movement.MovementComplete`
  (`self.FinishedMoving`))

(event `/Game/GeneralLogic/BPI_Damageable.ApplyDamage`
  (params (DamageInfo :type "/Game/GeneralLogic/S_DamageInfo Structure") (DamageCauser :type "Actor Object Reference"))
  (bind (_damagetype _damageamount _tickinterval _tickamount _knockbackforce _impactlocation) (break `/Game/GeneralLogic/S_DamageInfo` DamageInfo))
  (if (> (`self.currentHealth`) 0.0)
    (`self.ApplyKnockback` _impactlocation _knockbackforce)
    (bind _abovezero (`self.ReduceHealth` (* _damageamount (`self.BloodDamageModifier`))))
    (if _abovezero
      (`NiagaraFunctionLibrary.SpawnSystemAtLocation` "/Game/Enemies/VFX/Hit_FX/NS_Enemy_Hit_Neutral.NS_Enemy_Hit_Neutral" (`self.K2_GetActorLocation`))
      (`GameplayStatics.PlaySoundAtLocation` "/Game/Audio/SFX/A_EnemyHit_Cue.A_EnemyHit_Cue" (`self.K2_GetActorLocation`) (struct) 1.0 (`KismetMathLibrary.RandomFloatInRange` 0.8 1.2) 0.0 "/Game/Audio/SFX/Attenuation/ChaserSoundAttenuation.ChaserSoundAttenuation" null null null)
      (switch `/Game/GeneralLogic/E_DamageType` (`.DamageType_2_18CE76034A597327DFABC1A3DDE03055` (break `/Game/GeneralLogic/S_DamageInfo` DamageInfo))
        (:`NewEnumerator1`
          (`/Game/Enemies/BaseLogic/MLIB_EnemyBase.LightningStun` DamageInfo))
        (:`NewEnumerator2`
          (`/Game/Enemies/BaseLogic/MLIB_EnemyBase.PoisonDot` DamageInfo
            (:`Die`
              (`self.Die Event`)))))
      (else
        (`self.Die Event`)))))

(event `self.Die Event`
  (`parent.Die Event`)
  (`/Engine/EditorBlueprintResources/StandardMacros.DoOnce` false
    (:`Completed`
      (`self.Die` self)
      (`PrimitiveComponent.SetCollisionResponseToChannel` (`self.CapsuleComponent`) "ECC_Pawn" "ECR_Ignore")
      (`self.K2_DestroyActor`))))

(event `DissolveEvent`
  (bind _dissolveamount (`self.DissolveAmount`))
  (`MaterialInstanceDynamic.SetScalarParameterValue` (`self.DynamicMaterial`) "Dissolve" _dissolveamount)
  (set `self.DissolveAmount` (- _dissolveamount 0.1)))

(fn `ApplyKnockback`
  (params (`Hit Location` :type "Vector Structure") (KnockbackAmount :type "Float (double-precision)"))
  (bind (_returnvalue_x _returnvalue_y) (`KismetMathLibrary.BreakVector` (`KismetMathLibrary.Normal` (- (`self.K2_GetActorLocation`) `Hit Location`))))
  (`CharacterMovementComponent.AddImpulse` (`self.CharacterMovement`) (* (`KismetMathLibrary.MakeVector` _returnvalue_x _returnvalue_y 0.4) KnockbackAmount) true))

(fn `CalculateProjectileArcByVelocity`
  (params (Start :type "Vector Structure") (Goal :type "Vector Structure") (Speed :type "Float (double-precision)") (`Gravity Z Override` :type "Float (double-precision)" :default 980.0))
  (returns (LaunchVelocity :type "Vector Structure"))
  (locals (TempDirectionToTarget :type "Vector Structure"))
  (bind (_tempdirectiontotarget_x _tempdirectiontotarget_y) (`KismetMathLibrary.BreakVector` (`local.TempDirectionToTarget`)))
  (bind (_tempdirectiontotarget_x_2 _tempdirectiontotarget_y_2) (`KismetMathLibrary.BreakVector` (`local.TempDirectionToTarget`)))
  (bind (_tempdirectiontotarget_x_3 _tempdirectiontotarget_y_3 _tempdirectiontotarget_z) (`KismetMathLibrary.BreakVector` (`local.TempDirectionToTarget`)))
  (bind _speed (`local.Speed`))
  (set `local.TempDirectionToTarget` (- Goal Start))
  (return (+ (* (`KismetMathLibrary.Normal` (`KismetMathLibrary.MakeVector` _tempdirectiontotarget_x _tempdirectiontotarget_y)) (`local.Speed`)) (`KismetMathLibrary.MakeVector` 0.0 0.0 (+ _tempdirectiontotarget_z (* (/ (`KismetMathLibrary.Sqrt` (+ (`KismetMathLibrary.Square` (/ _tempdirectiontotarget_x_2 (`local.Speed`))) (`KismetMathLibrary.Square` (/ _tempdirectiontotarget_y_2 (`local.Speed`))))) 2.0) (/ (`local.Gravity Z Override`) _speed) _speed))))))

(fn `GetAttackablePosition`
  (params (TargetActor :type "Actor Object Reference"))
  (returns (AttackPosition :type "Vector Structure"))
  (bind (_returnvalue_x _returnvalue_y _returnvalue_z) (`KismetMathLibrary.BreakVector` (`self.K2_GetActorLocation` TargetActor)))
  (bind (_returnvalue_x_2 _returnvalue_y_2) (`KismetMathLibrary.BreakVector` (- (`self.K2_GetActorLocation`) (`self.K2_GetActorLocation` TargetActor))))
  (return (+ (* (`KismetMathLibrary.Normal` (`KismetMathLibrary.MakeVector` _returnvalue_x_2 _returnvalue_y_2) 0.01) (`self.attackRange`)) (`KismetMathLibrary.MakeVector` 0.0 0.0 (+ _returnvalue_z 100.0)))))

(fn `GetWorldPosition`
  (returns (RetVal :type "Vector Structure"))
  (return (`self.K2_GetActorLocation`)))

(fn `SetValuesFromStatComponent`
  (bind _stats_component (`self.Stats_Component`))
  (set `self.maxHealth` (`/Game/Enemies/BaseLogic/BP_EnemyBase_Stats_Component.MaxHealth` _stats_component))
  (set `self.baseDamage` (`/Game/Enemies/BaseLogic/BP_EnemyBase_Stats_Component.Base Damage` _stats_component))
  (set `self.attackRange` (`/Game/Enemies/BaseLogic/BP_EnemyBase_Stats_Component.AttackRange` _stats_component))
  (set `self.attacksPerSecond` (`/Game/Enemies/BaseLogic/BP_EnemyBase_Stats_Component.AttacksPerSecond` _stats_component))
  (set `self.reactionTime` (`/Game/Enemies/BaseLogic/BP_EnemyBase_Stats_Component.ReactionTime` _stats_component))
  (set `self.looseAggroTime` (`/Game/Enemies/BaseLogic/BP_EnemyBase_Stats_Component.LooseAggroTime` _stats_component))
  (set `self.movementSpeed` (`/Game/Enemies/BaseLogic/BP_EnemyBase_Stats_Component.MovementSpeed` _stats_component))
  (set `self.maxDistanceToWanderOfIdle` (`/Game/Enemies/BaseLogic/BP_EnemyBase_Stats_Component.MaxDistanceToWanderOfIdle` _stats_component))
  (set `self.RetreatRange` (`/Game/Enemies/VomiterFlying/Logic/BPC_EnemyVomiter_Flying_Stats.RetreatRange` _stats_component))
  (set `self.BulletSpread` (`/Game/Enemies/VomiterFlying/Logic/BPC_EnemyVomiter_Flying_Stats.BulletSpread` _stats_component))
  (set `self.targetables` (`/Game/Enemies/BaseLogic/BP_EnemyBase_Stats_Component.TargetableActorClasses` _stats_component))
  (if (not (>= (`self.FastGemDropWeight`) 0))
    (set `self.FastGemDropWeight` (`/Game/Enemies/BaseLogic/BP_EnemyBase_Stats_Component.FastGemDropWeight` _stats_component)))
  (if (not (>= (`self.HeavyGemDropWeight`) 0))
    (set `self.HeavyGemDropWeight` (`/Game/Enemies/BaseLogic/BP_EnemyBase_Stats_Component.HeavyGemDropWeight` _stats_component)))
  (if (not (>= (`self.MovementGemDropWeight`) 0))
    (set `self.MovementGemDropWeight` (`/Game/Enemies/BaseLogic/BP_EnemyBase_Stats_Component.MovementGemDropWeight` _stats_component)))
  (if (not (>= (`self.NullDropWeight`) 0))
    (set `self.NullDropWeight` (`/Game/Enemies/BaseLogic/BP_EnemyBase_Stats_Component.NullDropWeight` _stats_component))))

(fn `SuggestLaunchVelocity`
  (params (`Target Actor` :type "Actor Object Reference"))
  (returns (`Launch Velocity` :type "Vector Structure"))
  (bind _bulletspread (`/Game/Enemies/VomiterFlying/Logic/BPC_EnemyVomiter_Flying_Stats.BulletSpread` (`self.Stats_Component`)))
  (bind _returnvalue (* _bulletspread -1.0))
  (bind _outlaunchvelocity (`GameplayStatics.SuggestProjectileVelocity_CustomArc` (+ (`self.ShootPosition`) (`self.K2_GetActorLocation`)) (+ (`self.K2_GetActorLocation` `Target Actor`) (`KismetMathLibrary.MakeVector` (`KismetMathLibrary.RandomFloatInRange` _returnvalue _bulletspread) (`KismetMathLibrary.RandomFloatInRange` _returnvalue _bulletspread) (`KismetMathLibrary.RandomFloatInRange` _returnvalue _bulletspread))) 0.0 (`/Game/Enemies/VomiterFlying/Logic/BPC_EnemyVomiter_Flying_Stats.BulletArcModifier` (`self.Stats_Component`))))
  (return _outlaunchvelocity))

(fn `UserConstructionScript`)
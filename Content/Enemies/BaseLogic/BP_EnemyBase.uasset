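; Base enemy Blueprint that handles gem drops on death, a temporary blood damage modifier and hit stun.
; On death, a weighted roll picks a fast, heavy, movement or empty drop, then spawns that gem with a type differing from the player's equipped one.
; Rain of Blood raises the modifier once until its timer resets it.
; Each ApplyDamage restarts a timer that clears the stunned flag.
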(event `self.ReceiveBeginPlay`
  (add `self.Die` (delegate `Drop Gem On Death Event`)))

(event `Drop Gem On Death Event` :!signature `self.Die`
  (params (Actor :type "Actor Object Reference"))
  (bind _asbp_player_character (cast `/Game/Player/Logic/BP_PlayerCharacter` (`GameplayStatics.GetPlayerPawn` 0)))
  (bind _success (`self.Try Drop Gem` _asbp_player_character))
  (`KismetSystemLibrary.PrintString` (`KismetStringLibrary.Conv_BoolToString` _success)))

(event `ApplyRainOfBlood`
  (params (DamageIncrease :type "Float (double-precision)") (Duration :type "Float (double-precision)"))
  (`/Engine/EditorBlueprintResources/StandardMacros.DoOnce` false :!label _label
    (:`Completed`
      (set `self.BloodDamageModifier` (+ DamageIncrease (`self.BloodDamageModifier`)))
      (`KismetSystemLibrary.K2_SetTimerDelegate` (delegate `RemoveRainOfBlood`) Duration))))

(event `RemoveRainOfBlood`
  (set `self.BloodDamageModifier` 1.0)
  (goto _label :!via `Reset`))

(event `Die Event`)

(event `/Game/GeneralLogic/BPI_Damageable.ApplyDamage`
  (params (DamageInfo :type "/Game/GeneralLogic/S_DamageInfo Structure") (DamageCauser :type "Actor Object Reference"))
  (if (`KismetSystemLibrary.K2_TimerExistsHandle` (`self.DamageTakenTimer`))
    (`KismetSystemLibrary.K2_ClearAndInvalidateTimerHandle` (`self.DamageTakenTimer`)))
  (bind _returnvalue (`KismetSystemLibrary.K2_SetTimerDelegate` (delegate `ResetDamageTakenStunnedEvent`) (`self.DamageStunDuration`)))
  (set `self.DamageTakenTimer` _returnvalue)
  (set `self.DamageTakenStunned` true))

(event `ResetDamageTakenStunnedEvent`
  (set `self.DamageTakenStunned` false))

(fn `DropGem`
  (params (Slot :type "/Game/Player/Logic/E_GemSlot Enum" :default "NewEnumerator0") (Type :type "/Game/GeneralLogic/E_DamageType Enum" :default "NewEnumerator0"))
  (`|SpawnActorFromClass` (`|GetArrayItem` (`self.GemClasses`) (`KismetMathLibrary.Conv_ByteToInt` Slot)) (`KismetMathLibrary.MakeTransform` (`self.K2_GetActorLocation`) (`KismetMathLibrary.MakeRotator` 0.0 0.0 (`KismetMathLibrary.RandomFloatInRange` 0.0 360.0))) "Undefined" "MultiplyWithRoot" null Type null)
  (return))

(fn `Get Random Slot`
  (returns (Slot :type "/Game/Player/Logic/E_GemSlot Enum") (Success :type Boolean))
  (locals (RandomValue :type Integer) (Slot :type "/Game/Player/Logic/E_GemSlot Enum"))
  (bind _returnvalue (+ (`KismetMathLibrary.Clamp` (`self.FastGemDropWeight`) 0 2000000) (`KismetMathLibrary.Clamp` (`self.HeavyGemDropWeight`) 0 2000000) (`KismetMathLibrary.Clamp` (`self.MovementGemDropWeight`) 0 2000000) (`KismetMathLibrary.Clamp` (`self.NullDropWeight`) 0 2000000)))
  (if (> _returnvalue 0)
    (bind _output_get (set `local.RandomValue` (`KismetMathLibrary.RandomIntegerInRange` 1 _returnvalue)))
    (if (<= _output_get (+ (`self.FastGemDropWeight`) (`self.HeavyGemDropWeight`) (`self.MovementGemDropWeight`)))
      (if (<= (`local.RandomValue`) (+ (`self.FastGemDropWeight`) (`self.HeavyGemDropWeight`)))
        (if (<= (`local.RandomValue`) (`self.FastGemDropWeight`))
          (return "NewEnumerator0" true)
          (else
            (return "NewEnumerator1" true)))
        (else
          (return "NewEnumerator2" true)))
      (else
        (return "NewEnumerator0" false)))))

(fn `GetRandomGem`
  (params (Player :type "/Game/Player/Logic/BP_PlayerCharacter Object Reference") (Slot :type "/Game/Player/Logic/E_GemSlot Enum" :default "NewEnumerator0"))
  (returns (Gem :type "/Game/GeneralLogic/E_DamageType Enum"))
  (locals (DamageType :type "/Game/GeneralLogic/E_DamageType Enum") (RandomInt :type Integer))
  (bind _bpc_playerstats (`/Game/Player/Logic/BP_PlayerCharacter.BPC_PlayerStats` Player))
  (switch `/Game/Player/Logic/E_GemSlot` Slot
    (:`NewEnumerator0`
      (set `local.DamageType` (`/Game/Player/Logic/BPC_PlayerStats.GemFastSlot` _bpc_playerstats)))
    (:`NewEnumerator1`
      (set `local.DamageType` (`/Game/Player/Logic/BPC_PlayerStats.GemHeavySlot` _bpc_playerstats)))
    (:`NewEnumerator2`
      (set `local.DamageType` (`/Game/Player/Logic/BPC_PlayerStats.GemMovementSlot` _bpc_playerstats))))
  (bind _output_get (set `local.RandomInt` (`KismetMathLibrary.RandomIntegerInRange` 1 2)))
  (if (== _output_get (`KismetMathLibrary.Conv_ByteToInt` (`local.DamageType`)))
    (switch `int` (`local.RandomInt`)
      (:`1`
        (set `local.RandomInt` 2))
      (:`2`
        (set `local.RandomInt` 1))))
  (return (cast `/Game/GeneralLogic/E_DamageType` (`KismetMathLibrary.Conv_IntToByte` (`local.RandomInt`)))))

(fn `GetWorldPosition`
  (returns (RetVal :type "Vector Structure"))
  (return (0.0 0.0 0.0)))

(fn `Try Drop Gem`
  (params (Player :type "/Game/Player/Logic/BP_PlayerCharacter Object Reference"))
  (returns (Success :type Boolean))
  (locals (RandomFloat :type "Float (double-precision)" :default 0.0) (DamageType :type "/Game/GeneralLogic/E_DamageType Enum") (Slot :type "/Game/Player/Logic/E_GemSlot Enum"))
  (bind (_slot _success) (`self.Get Random Slot`))
  (if _success
    (bind _output_get (set `local.Slot` _slot))
    (`self.DropGem` _output_get (`self.GetRandomGem` (`local.Player`) (`local.Slot`)))
    (return true)
    (else
      (return false))))

(fn `UserConstructionScript`)
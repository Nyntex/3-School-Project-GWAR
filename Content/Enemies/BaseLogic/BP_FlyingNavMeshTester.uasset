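; Test flying enemy character that wanders between random positions to exercise flying nav mesh movement.
; On BeginPlay it binds to the FlyingMovement component's move-complete event, then after short delays asks that component for a random move.
; An older manual approach remains but is disconnected: NavMesh path requests with timer retries, plus waypoint following through movement input and distance thresholds.
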(event `self.ReceiveBeginPlay`
  (add `/Game/Enemies/BaseLogic/BP_FlyingMovement_Component.MovementComplete` (`self.Flying Movement`) (`|CreateDelegate` :!event `MoveToRandomPosition`))
  (`KismetSystemLibrary.Delay` 0.2)
  (`self.MoveToRandomPosition`))

(event `MoveToRandomPosition`
  (`KismetSystemLibrary.Delay` 0.2)
  (`/Game/Enemies/BaseLogic/BP_FlyingMovement_Component.MoveToRandomPosition` (`self.Flying Movement`)))

(event `self.ReceiveTick`
  (params (DeltaSeconds :type "Float (single-precision)")))

(event `GetNewPath`
  (bind _navmesh (`self.NavMesh`)
    (:`then`
      (bind _path (`HeightNavigationVolume.GetPath` _navmesh (`self.K2_GetActorLocation`) null (`HeightNavigationVolume.GetRandomMovablePosition` _navmesh) null)
        (:`Success`
          (set `self.Path` _path)
          (set `self.pathCounter` 0))
        (:`Failed`
          (bind _returnvalue (`KismetSystemLibrary.K2_SetTimerDelegate` (delegate `GetNewPath`) 2.0 false 0.0 0.2))
          (set `self.NewPathTimer` _returnvalue))))
    (:`else`)))

(fn `Get Direction Position`
  (params (Position :type "Vector Structure"))
  (returns (ReturnValue :type "Vector Structure"))
  (return (`KismetMathLibrary.Normal` (- Position (`self.K2_GetActorLocation`)))))

(fn `IsBelowThreshold`
  (params (Threshold :type "Float (double-precision)"))
  (returns (ReturnValue :type Boolean))
  (return (<= (`KismetMathLibrary.Vector_Distance` (`self.LastPositionToMoveTo`) (`self.K2_GetActorLocation`)) Threshold)))

(fn `IsCloseEnough`
  (returns (ReturnValue :type Boolean))
  (return (<= (`KismetMathLibrary.Vector_Distance` (`|GetArrayItem` (`self.Path`)) (`self.K2_GetActorLocation`)) 250.0)))

(fn `IsMoveInsideNavMesh`
  (returns (IsInside :type Boolean))
  (return (`HeightNavigationVolume.IsInsideVolume` (`self.NavMesh`) (+ (`self.K2_GetActorLocation`) (* (`self.CurrentDirection`) 100.0)))))

(fn `MoveToPosition`
  (params (Position :type "Vector Structure"))
  (if (`KismetMathLibrary.NotEqualExactly_VectorVector` Position (`self.K2_GetActorLocation`))
    (`self.AddMovementInput` (`self.Get Direction Position` Position))
    (return)))

(fn `RotateToMoveDirection`
  (params (Direction :type "Vector Structure"))
  (bind _returnvalue (`self.K2_GetActorLocation`))
  (bind (_returnvalue_roll _returnvalue_pitch _returnvalue_yaw) (`KismetMathLibrary.BreakRotator` (`KismetMathLibrary.FindLookAtRotation` _returnvalue (+ Direction _returnvalue))))
  (`self.K2_SetActorRotation` (`KismetMathLibrary.MakeRotator` 0.0 0.0 _returnvalue_yaw)))

(fn `UserConstructionScript`)
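; Big Chaser enemy that wanders around its start point when idle, chases the closest targetable actor and makes delayed, range-checked melee attacks.
; Stats are copied from a stat component at BeginPlay, after which that component is destroyed.
; Damage applies knockback, a temporary health bar and type-specific effects like lightning stun and poison damage over time.
; Death plays a montage whose notify starts a timer-driven, damage-tinted material dissolve before destroying the actor.
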(event `self.ReceiveTick`
  (params (DeltaSeconds :type "Float (single-precision)"))
  (bind _targetableactors (`self.targetableActors`))
  (`parent.ReceiveTick` DeltaSeconds)
  (if (`KismetArrayLibrary.Array_IsEmpty` _targetableactors)
    (set `self.possibleTarget` null)
    (else
      (set `self.possibleTarget` (`self.GetClosestActor` _targetableactors))))
  (`self.TryDisableHealthWidgetOutsideOfVisibleRange`))

(event `self.ReceiveBeginPlay`
  (`parent.ReceiveBeginPlay`)
  ;[1 0 0] Health Bar Hide On Default
  (`SceneComponent.SetVisibility` (`self.Health Bar Widget`) false false)
  (`self.SetValuesFromStatComponent`)
  (bind _asabp_enemy (cast `/Game/Enemies/Chaser/Animation/ABP_Enemy` (`SkeletalMeshComponent.GetAnimInstance` (`self.Mesh`))))
  (set `self.AnimInstance` _asabp_enemy)
  (`KismetSystemLibrary.Delay` 0.2)
  (`GameplayStatics.SpawnSoundAttached` "/Game/Audio/SFX/MetaSounds/MS_BigEnemyIdle.MS_BigEnemyIdle" (`self.CapsuleComponent`) "None" (0.0 0.0 0.0) (struct) "KeepRelativeOffset" true 1.0 1.0 0.0 null null)
  (`KismetMaterialLibrary.SetScalarParameterValue` "/Game/GeneralVFX/MPC_NewMaterialParameterCollection.MPC_NewMaterialParameterCollection" "Dissolve" 0.5)
  (bind _returnvalue (`PrimitiveComponent.CreateDynamicMaterialInstance` (`self.Mesh`) 0 "/Game/Enemies/Chaser/Effects/MI_EnemyDeath_Lightning_Inst.MI_EnemyDeath_Lightning_Inst" "None"))
  (bind _output_get (set `self.DynamicMaterial` _returnvalue))
  (`MaterialInstanceDynamic.SetScalarParameterValue` _output_get "Dissolve" 0.5)
  (`MaterialInstanceDynamic.SetScalarParameterValue` (`self.DynamicMaterial`) "Hue" (* (`KismetMathLibrary.RandomFloatInRange` -7.5 7.5) 0.01))
  (`SceneComponent.SetRelativeScale3D` (`self.CapsuleComponent`) (`KismetMathLibrary.Conv_DoubleToVector` (`KismetMathLibrary.RandomFloatInRange` 0.9 1.1))))

(event `Move`
  (switch `EEnemyStates` (`self.currentState`)
    (:`IDLE`
      (`self.MoveIdle`))
    (:`CHASE`
      (`self.MoveChase`))))

(event `MoveIdle`
  (if (`self.Stunned`)
    (`NavMovementComponent.StopActiveMovement` (`self.CharacterMovement`))
    (else
      (`/Engine/EditorBlueprintResources/StandardMacros.DoOnce` false :!label _label
        (:`Completed`
          (bind (_randomlocation _returnvalue) (`NavigationSystemV1.K2_GetRandomLocationInNavigableRadius` (`self.startPosition`) (`self.maxDistanceToWanderOfIdle`) null null))
          (if _returnvalue
            (`|AIMoveTo` self _randomlocation null 25.0
              (:`OnSuccess`
                _)
              (:`OnFail`
                _))
            (else
              (`|AIMoveTo` self (`self.startPosition`) null 25.0
                (:`OnSuccess`
                  _)
                (:`OnFail`
                  _))))
          (`KismetSystemLibrary.Delay` 0.0)
          (`self.FinishedMoving`)
          (goto _label :!via `Reset`))))))

(event `MoveChase`
  (bind _targetableactors (`self.targetableActors`))
  (if (`self.Stunned`)
    (`NavMovementComponent.StopActiveMovement` (`self.CharacterMovement`))
    (else
      (`/Engine/EditorBlueprintResources/StandardMacros.DoOnce` false :!label _label_2
        (:`Completed`
          (if (not (`KismetArrayLibrary.Array_IsEmpty` _targetableactors))
            (`|AIMoveTo` self (0.0 0.0 0.0) (`self.GetClosestActor` _targetableactors) (* (`self.attackRange`) 0.5)
              (:`OnSuccess`
                _)
              (:`OnFail`
                _))
            (`KismetSystemLibrary.Delay` 0.0)
            (`self.FinishedMoving`)
            (goto _label_2 :!via `Reset`)))))))

(event `Event ChangeState`
  (params (State :type "EEnemyStates Enum" :default "Invalid"))
  (`self.ChangeState` State))

(event `Event TryAttack`
  (params (AttackTarget :type "Actor Object Reference"))
  (if (not (`self.DamageTakenStunned`))
    (`/Engine/EditorBlueprintResources/StandardMacros.DoOnce` false :!label _label_3
      (:`Completed`
        (if (`.inRange` (`self.IsActorInAttackRange` AttackTarget))
          (`/Game/Enemies/Chaser/Animation/ABP_Enemy.StartAttack` (`self.AnimInstance`))
          (`KismetSystemLibrary.Delay` (/ 0.5 (`self.attacksPerSecond`)))
          (if (not (`self.DamageTakenStunned`))
            (if (<= (`self.GetDistanceTo` AttackTarget) (`self.AttackAnimationBonusRange`))
              (bind _asbpi_damageable (cast `/Game/GeneralLogic/BPI_Damageable` AttackTarget)
                (:`then`
                  (`/Game/GeneralLogic/BPI_Damageable.ApplyDamage` _asbpi_damageable (make `/Game/GeneralLogic/S_DamageInfo` "NewEnumerator0" (`self.baseDamage`) 0.0 0.0 0.0 (`self.K2_GetActorLocation`)) self))
                (:`CastFailed`
                  (`GameplayStatics.ApplyDamage` AttackTarget (`self.baseDamage`) null self)))
              (`GameplayStatics.PlaySoundAtLocation` "/Game/Audio/SFX/MetaSounds/MS_BigEnemyAttack.MS_BigEnemyAttack" (`self.K2_GetActorLocation`) (struct) 1.0 (`KismetMathLibrary.RandomFloatInRange` 0.9 1.1) 0.0 null null null null)
              (`KismetSystemLibrary.Delay` (* (- (`self.attacksPerSecond`) (/ 0.5 (`self.attacksPerSecond`))) (`KismetMathLibrary.RandomFloatInRange` 0.8 1.2))))))
        (`|ExecutionSequence`
          (:`then_0`
            (goto _label_3 :!via `Reset`))
          (:`then_1`
            (`self.FinishedAttacking`)))))
    (else
      (`self.FinishedAttacking`))))

(event `self.ApplyDamage`
  (params (DamageInfo :type "/Game/GeneralLogic/S_DamageInfo Structure") (DamageCauser :type "Actor Object Reference"))
  (bind (_damagetype _damageamount _tickinterval _tickamount _knockbackforce _impactlocation) (break `/Game/GeneralLogic/S_DamageInfo` DamageInfo))
  (if (> (`self.currentHealth`) 0.0)
    (set `self.LastHitDamageType` _damagetype)
    (`self.ApplyKnockback` _impactlocation _knockbackforce)
    (if (> _knockbackforce 500.0)
      (`AddComponent|NODE_AddBPC_KickedBehaviour-0`))
    (bind _abovezero (`self.ReduceHealth` (* _damageamount (`self.BloodDamageModifier`))))
    ;[1 0 0] Update Health Bar
    (`self.Update HP Bar`)
    (if _abovezero
      (`/Game/Enemies/Chaser/Animation/ABP_Enemy.GetHit` (`self.AnimInstance`))
      (`NiagaraFunctionLibrary.SpawnSystemAtLocation` (select `/Game/GeneralLogic/E_DamageType` (`self.LastHitDamageType`) :`NewEnumerator0` "/Game/Enemies/VFX/Hit_FX/NS_Enemy_Hit_Blood.NS_Enemy_Hit_Blood" :`NewEnumerator1` "/Game/Enemies/VFX/Hit_FX/NS_Enemy_Hit_Lightning.NS_Enemy_Hit_Lightning" :`NewEnumerator2` "/Game/Enemies/VFX/Hit_FX/NS_Enemy_Hit_Poison.NS_Enemy_Hit_Poison" :`NewEnumerator4` "/Game/Enemies/VFX/Hit_FX/NS_Enemy_Hit_Blood.NS_Enemy_Hit_Blood" :`NewEnumerator5` "/Game/Enemies/VFX/Hit_FX/NS_Enemy_Hit_Magic.NS_Enemy_Hit_Magic" :!type "NiagaraSystem Object Reference") (`self.K2_GetActorLocation`))
      (`GameplayStatics.PlaySoundAtLocation` "/Game/Audio/SFX/MetaSounds/MS_BigEnemyTakesDamage.MS_BigEnemyTakesDamage" (`self.K2_GetActorLocation`) (struct) 1.0 (`KismetMathLibrary.RandomFloatInRange` 0.8 1.2) 0.0 "/Game/Audio/SFX/Attenuation/ChaserSoundAttenuation.ChaserSoundAttenuation" null null null)
      (switch `/Game/GeneralLogic/E_DamageType` (`.DamageType_2_18CE76034A597327DFABC1A3DDE03055` (break `/Game/GeneralLogic/S_DamageInfo` DamageInfo))
        (:`NewEnumerator0`
          ;[1 0 0] Hide Health Bar
          (`KismetSystemLibrary.Delay` 10.0 :!label _label_4)
          (`SceneComponent.SetVisibility` (`self.Health Bar Widget`) false false :!label _label_5))
        (:`NewEnumerator1`
          (`self.FinishedMoving`)
          (`/Game/Enemies/BaseLogic/MLIB_EnemyBase.LightningStun` DamageInfo
            (:`Finished`
              (goto _label_4))))
        (:`NewEnumerator2`
          (`/Game/Enemies/BaseLogic/MLIB_EnemyBase.PoisonDot` DamageInfo
            (:`Finished`
              (goto _label_4))
            (:`Die`
              (`self.Die Event`)
              (goto _label_5))
            (:`PerTick`
              (`self.Update HP Bar`))))
        (:`NewEnumerator4`
          (goto _label_4))
        (:`NewEnumerator5`
          (goto _label_4)))
      (else
        (`self.Die Event`)
        (goto _label_5)))))

(event `self.Die Event`
  (`/Engine/EditorBlueprintResources/StandardMacros.DoOnce` false
    (:`Completed`
      (`parent.Die Event`)
      (`self.Die` self)
      (`PrimitiveComponent.SetCollisionResponseToChannel` (`self.CapsuleComponent`) "ECC_Pawn" "ECR_Ignore")
      (`|PlayMontage` (`self.Mesh`) "/Game/Enemies/Chaser/Animation/AM_Enemy_Death.AM_Enemy_Death"
        (:`then`
          (`GameplayStatics.PlaySoundAtLocation` "/Game/Audio/SFX/MetaSounds/MS_BigEnemyDeath.MS_BigEnemyDeath" (`self.K2_GetActorLocation`) (struct) 1.0 1.0 0.0 null null null null)
          (`NiagaraFunctionLibrary.SpawnSystemAttached` (select `/Game/GeneralLogic/E_DamageType` (`self.LastHitDamageType`) :`NewEnumerator4` "/Game/Enemies/VFX/Death_FX/NS_Enemy_Death_Blood.NS_Enemy_Death_Blood" :`NewEnumerator5` "/Game/Enemies/VFX/Death_FX/NS_Enemy_Death_Magic.NS_Enemy_Death_Magic" :!type "NiagaraSystem Object Reference") (`self.Mesh`) "None" (0.0 0.0 0.0) (struct) "KeepRelativeOffset")
          (`SceneComponent.SetVisibility` (`self.StunnedMesh`) false false))
        (:`OnBlendOut`
          (`KismetSystemLibrary.K2_ClearAndInvalidateTimerHandle` (`self.DissolveTimer`))
          (`self.K2_DestroyActor`))
        (:`OnNotifyBegin`
          (`NiagaraFunctionLibrary.SpawnSystemAttached` (select `/Game/GeneralLogic/E_DamageType` (`self.LastHitDamageType`) :`NewEnumerator0` "/Game/Enemies/VFX/Death_FX/NS_Enemy_Death_Neutral.NS_Enemy_Death_Neutral" :`NewEnumerator1` "/Game/Enemies/VFX/Death_FX/NS_Enemy_Death_Lightning.NS_Enemy_Death_Lightning" :`NewEnumerator2` "/Game/Enemies/VFX/Death_FX/NS_Enemy_Death_Poison.NS_Enemy_Death_Poison" :`NewEnumerator5` "/Game/Enemies/VFX/Death_FX/NS_Enemy_Death_Magic.NS_Enemy_Death_Magic" :!type "NiagaraSystem Object Reference") (`self.Mesh`) "None" (0.0 0.0 0.0) (struct) "KeepRelativeOffset")
          (`KismetSystemLibrary.Delay` 0.3)
          (bind _returnvalue (`KismetSystemLibrary.K2_SetTimerDelegate` (delegate `DissolveEvent`) 0.05 true))
          (set `self.DissolveTimer` _returnvalue)
          (`MaterialInstanceDynamic.SetVectorParameterValue` (`self.DynamicMaterial`) "Emissive Color" (select `/Game/GeneralLogic/E_DamageType` (`self.LastHitDamageType`) :`NewEnumerator1` (struct :`G` 0.180769 :`B` 1.0 :`A` 1.0) :`NewEnumerator2` (struct :`G` 1.0 :`B` 0.161287 :`A` 1.0) :`NewEnumerator4` (struct :`R` 1.0 :`B` 0.022203 :`A` 1.0) :`NewEnumerator5` (struct :`A` 1.0) :!type "LinearColor Structure")))))))

(event `DissolveEvent`
  (bind _dissolveamount (`self.DissolveAmount`))
  (`MaterialInstanceDynamic.SetScalarParameterValue` (`self.DynamicMaterial`) "Dissolve" _dissolveamount)
  (set `self.DissolveAmount` (- _dissolveamount 0.1)))

(fn `ApplyKnockback`
  (params (`Hit Location` :type "Vector Structure") (KnockbackAmount :type "Float (double-precision)"))
  (bind (_returnvalue_x _returnvalue_y) (`KismetMathLibrary.BreakVector` (`KismetMathLibrary.Normal` (- (`self.K2_GetActorLocation`) `Hit Location`))))
  (`CharacterMovementComponent.AddImpulse` (`self.CharacterMovement`) (* (`KismetMathLibrary.MakeVector` _returnvalue_x _returnvalue_y 0.4) KnockbackAmount) true))

(fn `GetWorldPosition`
  (returns (RetVal :type "Vector Structure"))
  (return (`self.K2_GetActorLocation`)))

(fn `SetValuesFromStatComponent`
  (bind _bpc_enemybigchaser_stats (`self.BPC_EnemyBigChaser_Stats`))
  (`|ExecutionSequence`
    (:`then_0`
      (set `self.maxHealth` (`/Game/Enemies/Chaser/Logic/BPC_EnemyChaser_Stats.MaxHealth` _bpc_enemybigchaser_stats))
      (set `self.attackRange` (`/Game/Enemies/Chaser/Logic/BPC_EnemyChaser_Stats.AttackRange` _bpc_enemybigchaser_stats))
      (set `self.attacksPerSecond` (`/Game/Enemies/Chaser/Logic/BPC_EnemyChaser_Stats.AttacksPerSecond` _bpc_enemybigchaser_stats))
      (set `self.baseDamage` (`/Game/Enemies/BaseLogic/BP_EnemyBase_Stats_Component.Base Damage` _bpc_enemybigchaser_stats))
      (set `self.reactionTime` (`/Game/Enemies/Chaser/Logic/BPC_EnemyChaser_Stats.ReactionTime` _bpc_enemybigchaser_stats))
      (set `self.looseAggroTime` (`/Game/Enemies/Chaser/Logic/BPC_EnemyChaser_Stats.LooseAggroTime` _bpc_enemybigchaser_stats))
      (set `self.maxDistanceToWanderOfIdle` (`/Game/Enemies/Chaser/Logic/BPC_EnemyChaser_Stats.MaxDistancetoWanderOfIdle` _bpc_enemybigchaser_stats))
      (set `self.targetables` (`/Game/Enemies/BaseLogic/BP_EnemyBase_Stats_Component.TargetableActorClasses` _bpc_enemybigchaser_stats))
      (set `self.DamageStunDuration` (`/Game/Enemies/BaseLogic/BP_EnemyBase_Stats_Component.DamageStunDuration` _bpc_enemybigchaser_stats))
      (set `self.HealthBarDisableRange` (`/Game/Enemies/BaseLogic/BP_EnemyBase_Stats_Component.HealthBarDisableRange` _bpc_enemybigchaser_stats))
      (set `self.AttackAnimationBonusRange` (`/Game/Enemies/Chaser/Logic/BPC_EnemyChaser_Stats.AttackAnimationBonusRange` _bpc_enemybigchaser_stats))
      (if (not (>= (`self.FastGemDropWeight`) 0))
        (set `self.FastGemDropWeight` (`/Game/Enemies/BaseLogic/BP_EnemyBase_Stats_Component.FastGemDropWeight` _bpc_enemybigchaser_stats)))
      (if (not (>= (`self.HeavyGemDropWeight`) 0))
        (set `self.HeavyGemDropWeight` (`/Game/Enemies/BaseLogic/BP_EnemyBase_Stats_Component.HeavyGemDropWeight` _bpc_enemybigchaser_stats)))
      (if (not (>= (`self.MovementGemDropWeight`) 0))
        (set `self.MovementGemDropWeight` (`/Game/Enemies/BaseLogic/BP_EnemyBase_Stats_Component.MovementGemDropWeight` _bpc_enemybigchaser_stats)))
      (if (not (>= (`self.NullDropWeight`) 0))
        (set `self.NullDropWeight` (`/Game/Enemies/BaseLogic/BP_EnemyBase_Stats_Component.NullDropWeight` _bpc_enemybigchaser_stats))))
    (:`then_1`
      (`ActorComponent.K2_DestroyComponent` (`self.BPC_EnemyBigChaser_Stats`)))))

(fn `TryDisableHealthWidgetOutsideOfVisibleRange`
  (if (> (`KismetMathLibrary.Vector_Distance` (`self.K2_GetActorLocation` (`GameplayStatics.GetPlayerCameraManager` 0)) (`self.K2_GetActorLocation`)) (`self.HealthBarDisableRange`))
    (`SceneComponent.SetVisibility` (`self.Health Bar Widget`) false false)))

(fn `Update HP Bar`
  (bind _asbp_enemy_health_bar (cast `/Game/Enemies/BaseLogic/BP_EnemyHealthBar` (`WidgetComponent.GetWidget` (`self.Health Bar Widget`))))
  (`ProgressBar.SetPercent` (`/Game/Enemies/BaseLogic/BP_EnemyHealthBar.EnemyHealthBar` _asbp_enemy_health_bar) (/ (`self.currentHealth`) (`self.maxHealth`)))
  (`SceneComponent.SetVisibility` (`self.Health Bar Widget`) true false))

(fn `UserConstructionScript`)
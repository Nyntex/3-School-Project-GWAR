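; BP_WeaponTest is a test Blueprint that fits an attack ribbon VFX component, NSPlayerAttackNeutral, to a weapon.
; SetSocketsLocations reads the weapon's TopSocket and BottomSocket positions, sets RibbonWidth to their distance, aligns the effect's Z axis along the blade and centers it between them.
; Within this graph the fit runs only on BeginPlay, with no per-frame update.
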(event `SetSocketsLocations`
  (bind _weapon (`self.Weapon`))
  (bind _output_get (set `self.TopPosition` (`SceneComponent.GetSocketLocation` _weapon "TopSocket")))
  (bind _output_get_2 (set `self.BottomPosition` (`SceneComponent.GetSocketLocation` _weapon "BottomSocket")))
  (bind _returnvalue (- _output_get _output_get_2))
  (`FXSystemComponent.SetFloatParameter` (`self.NS_PlayerAttack_Neutral`) "RibbonWidth" (`KismetMathLibrary.VSize` _returnvalue))
  (`SceneComponent.K2_SetWorldRotation` (`self.NS_PlayerAttack_Neutral`) (`KismetMathLibrary.MakeRotFromZ` _returnvalue) false false)
  (`SceneComponent.K2_SetWorldLocation` (`self.NS_PlayerAttack_Neutral`) (/ (+ _output_get _output_get_2) 2) false false))

(event `self.ReceiveBeginPlay`
  (`self.SetSocketsLocations`))

(fn `UserConstructionScript`)
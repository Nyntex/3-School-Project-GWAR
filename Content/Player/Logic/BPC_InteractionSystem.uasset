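; Player component that detects, highlights and picks up gem pickups for the fast, heavy and movement slots.
; Every 0.1 seconds it traces along the camera forward, sphere-overlaps at the hit or trace end, and highlights the closest gem, with a one-time pausing popup.
; Pickup writes the gem to BPC_PlayerStats, updates character gem meshes and saves to the game instance, which restores slots on BeginPlay.
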(event `self.ReceiveTick`
  (params (DeltaSeconds :type "Float (single-precision)")))

(event `self.ReceiveBeginPlay`
  (bind _asbp_player_character (cast `/Game/Player/Logic/BP_PlayerCharacter` (`self.GetOwner`)))
  (set `self.As BP Player Character` _asbp_player_character)
  (`self.GetSavedGems`)
  (`self.ReloadGemMeshes`)
  (`KismetSystemLibrary.Delay` 0.1 :!label _label)
  (`self.Check Gems`)
  (goto _label))

(event `Check Gems`
  (bind _returnvalue (`GameplayStatics.GetPlayerController` 0))
  (bind (_returnvalue_2 _outhitactors _impactposition) (`self.FindActorsInInteractionRange`))
  (if _returnvalue_2
    (bind _gems (`self.GetGemsFromHitActors` _outhitactors))
    (if (> (`KismetArrayLibrary.Array_Length` _gems) 0)
      (`|ExecutionSequence`
        (:`then_0`
          (`self.HighlightClosestGem` _gems _impactposition))
        (:`then_1`
          (`/Engine/EditorBlueprintResources/StandardMacros.DoOnce` false
            (:`Completed`
              (bind _asbp_game_instance (cast `/Game/GeneralLogic/BP_GameInstance` (`GameplayStatics.GetGameInstance`)))
              (if (not (`/Game/GeneralLogic/BP_GameInstance.GemPopupShown` _asbp_game_instance))
                (bind _returnvalue_3 (`|CreateWidget` "/Game/UI/OtherWidgets/WBP_GemPopup.WBP_GemPopup_C" _returnvalue))
                (`UserWidget.AddToViewport` _returnvalue_3 0)
                (`GameplayStatics.SetGamePaused` true)
                (set `PlayerController.bShowMouseCursor` true _returnvalue)
                (set `/Game/GeneralLogic/BP_GameInstance.GemPopupShown` true _asbp_game_instance)))))))
    (else
      (`self.TryStopCurrentHighlight`))))

(event `Pick Up Gem`
  (bind _highlightedgem (`self.HighlightedGem`)
    (:`then`
      (`|ExecutionSequence`
        (:`then_0`
          (bind (_gemslottype _gemtype) (`/Game/GeneralLogic/Gems/BP_BaseGemPickup.Pickup` _highlightedgem))
          (`self.SetNewGem` _gemslottype _gemtype)
          (`self.OnPickup` _gemslottype _gemtype)
          (`self.ReloadGemMeshes`)
          (`self.SaveGems`)
          (`GameplayStatics.PlaySound2D` "/Game/Audio/SFX/MetaSounds/MS_GemAcquired.MS_GemAcquired" 1.0 1.0 0.0 null null))))
    (:`else`)))

(fn `FindActorsInInteractionRange`
  (returns (ReturnValue :type Boolean) (OutHitActors :type "Array of Actor Object Reference") (ImpactPosition :type "Vector Structure"))
  (bind _returnvalue (`Actor.GetComponentByClass` (`self.GetOwner`) "/Script/Engine.SpringArmComponent"))
  (bind _returnvalue_2 (`SceneComponent.K2_GetComponentLocation` _returnvalue))
  (`/Engine/EditorBlueprintResources/StandardMacros.IsValid` _returnvalue
    (:`Is Valid`
      (bind (_outhit _returnvalue_3) (`KismetSystemLibrary.LineTraceSingle` :`Start` _returnvalue_2 :`End` (+ _returnvalue_2 (* (`self.GetOwnerCameraForwardVector`) (`self.InteractionRange`))) :`TraceChannel` "TraceTypeQuery1" :`DrawDebugType` "ForDuration" :`DrawTime` 0.2))
      (if _returnvalue_3
        (bind (_bblockinghit _binitialoverlap _time _distance _location _impactpoint _normal _impactnormal _physmat _hitactor _hitcomponent _hitbonename _bonename _hititem _elementindex _faceindex _tracestart _traceend) (`GameplayStatics.BreakHitResult` _outhit))
        (bind (_outactors _returnvalue_4) (`KismetSystemLibrary.SphereOverlapActors` _location (`self.InteractionDetectionSize`) (`|MakeArray` "ObjectTypeQuery2" :!type "EObjectTypeQuery Enum")))
        (return _returnvalue_4 _outactors _location)
        (else
          (bind (_outactors_2 _returnvalue_5) (`KismetSystemLibrary.SphereOverlapActors` _traceend (`self.InteractionDetectionSize`) (`|MakeArray` "ObjectTypeQuery2" :!type "EObjectTypeQuery Enum")))
          (return _returnvalue_5 _outactors_2 _traceend))))
    (:`Is Not Valid`
      (return false _ (0.0 0.0 0.0)))))

(fn `GetGemsFromHitActors`
  (params (HitActors :type "Array of Actor Object Reference"))
  (returns (Gems :type "Array of /Game/GeneralLogic/Gems/BP_BaseGemPickup Object Reference"))
  (locals (TempGems :type "Array of /Game/GeneralLogic/Gems/BP_BaseGemPickup Object Reference"))
  (for _array_element HitActors
    (bind _asbp_base_gem_pickup (cast `/Game/GeneralLogic/Gems/BP_BaseGemPickup` _array_element))
    (`KismetArrayLibrary.Array_AddUnique` (`local.TempGems`) _asbp_base_gem_pickup))
  (return (`local.TempGems`)))

(fn `GetOwnerCameraForwardVector`
  (returns (ReturnValue :type "Vector Structure"))
  (return (`SceneComponent.GetForwardVector` (`Actor.GetComponentByClass` (`self.GetOwner`) "/Script/Engine.CameraComponent"))))

(fn `GetSavedGems`
  (bind _asbp_game_instance (cast `/Game/GeneralLogic/BP_GameInstance` (`GameplayStatics.GetGameInstance`)))
  (bind (_fastgem _heavygem _movementgem) (`/Game/GeneralLogic/BP_GameInstance.GetSavedGems` _asbp_game_instance))
  (`self.SetNewGem` "NewEnumerator0" _fastgem)
  (`self.SetNewGem` "NewEnumerator1" _heavygem)
  (`self.SetNewGem` "NewEnumerator2" _movementgem))

(fn `HighlightClosestGem`
  (params (Gems :type "Array of /Game/GeneralLogic/Gems/BP_BaseGemPickup Object Reference (by ref)") (CheckPosition :type "Vector Structure"))
  (bind _checkposition (`local.CheckPosition`))
  (bind _highlightedgem (`self.HighlightedGem`))
  (if (>= (`KismetArrayLibrary.Array_Find` Gems (`self.HighlightedGem`)) 0)
    (for _array_element (`local.Gems`) :!label _label
      (if (> (`KismetMathLibrary.Vector_Distance` (`Actor.K2_GetActorLocation` (`self.HighlightedGem`)) _checkposition) (`KismetMathLibrary.Vector_Distance` _checkposition (`Actor.K2_GetActorLocation` _array_element)))
        (`self.TryStopCurrentHighlight`)
        (set `self.HighlightedGem` _array_element)))
    (`/Game/GeneralLogic/Gems/BP_BaseGemPickup.Highlight` _highlightedgem)
    (`self.OnGemHighlight` (`/Game/GeneralLogic/Gems/BP_BaseGemPickup.GemSlotType` _highlightedgem) (`/Game/GeneralLogic/Gems/BP_BaseGemPickup.GemType` _highlightedgem))
    (else
      (`self.TryStopCurrentHighlight`)
      (if (> (`KismetArrayLibrary.Array_Length` (`local.Gems`)) 0)
        (set `self.HighlightedGem` (`|GetArrayItem` (`local.Gems`)))
        (goto _label)
        (else
          (set `self.HighlightedGem` null))))))

(fn `ReloadGemMeshes`
  (bind _as_bp_player_character (`self.As BP Player Character`))
  (bind _returnvalue (`Actor.GetComponentByClass` (`self.GetOwner`) "/Game/Player/Logic/BPC_PlayerStats.BPC_PlayerStats_C"))
  (bind _gemmovementslot (`/Game/Player/Logic/BPC_PlayerStats.GemMovementSlot` _returnvalue))
  (`|ExecutionSequence`
    (:`then_0`
      (`self.SetupGemMaterialByDamage` (`/Game/Player/Logic/BP_PlayerCharacter.FastGem` (`self.As BP Player Character`)) (`/Game/Player/Logic/BPC_PlayerStats.GemFastSlot` _returnvalue)))
    (:`then_1`
      (`self.SetupGemMaterialByDamage` (`/Game/Player/Logic/BP_PlayerCharacter.HeavyGem` (`self.As BP Player Character`)) (`/Game/Player/Logic/BPC_PlayerStats.GemHeavySlot` _returnvalue)))
    (:`then_2`
      (`self.SetupGemMaterialByDamage` (`/Game/Player/Logic/BP_PlayerCharacter.MovementGem1` _as_bp_player_character) _gemmovementslot)
      (`self.SetupGemMaterialByDamage` (`/Game/Player/Logic/BP_PlayerCharacter.MovementGem2` _as_bp_player_character) _gemmovementslot))))

(fn `SaveGems`
  (bind _returnvalue (`Actor.GetComponentByClass` (`self.GetOwner`) "/Game/Player/Logic/BPC_PlayerStats.BPC_PlayerStats_C"))
  (bind _asbp_game_instance (cast `/Game/GeneralLogic/BP_GameInstance` (`GameplayStatics.GetGameInstance`)))
  (set `/Game/GeneralLogic/BP_GameInstance.PlayerFastGem` (`/Game/Player/Logic/BPC_PlayerStats.GemFastSlot` _returnvalue) _asbp_game_instance)
  (set `/Game/GeneralLogic/BP_GameInstance.PlayerHeavyGem` (`/Game/Player/Logic/BPC_PlayerStats.GemHeavySlot` _returnvalue) _asbp_game_instance)
  (set `/Game/GeneralLogic/BP_GameInstance.PlayerMovementGem` (`/Game/Player/Logic/BPC_PlayerStats.GemMovementSlot` _returnvalue) _asbp_game_instance))

(fn `SetNewGem`
  (params (SlotType :type "/Game/Player/Logic/E_GemSlot Enum" :default "NewEnumerator0") (`Gem Type` :type "/Game/GeneralLogic/E_DamageType Enum" :default "NewEnumerator0"))
  (bind _returnvalue (`Actor.GetComponentByClass` (`self.GetOwner`) "/Game/Player/Logic/BPC_PlayerStats.BPC_PlayerStats_C"))
  (if (`|EnumInequality` `Gem Type` "NewEnumerator0")
    (switch `/Game/Player/Logic/E_GemSlot` SlotType
      (:`NewEnumerator0`
        (set `/Game/Player/Logic/BPC_PlayerStats.GemFastSlot` `Gem Type` _returnvalue))
      (:`NewEnumerator1`
        (set `/Game/Player/Logic/BPC_PlayerStats.GemHeavySlot` `Gem Type` _returnvalue))
      (:`NewEnumerator2`
        (set `/Game/Player/Logic/BPC_PlayerStats.GemMovementSlot` `Gem Type` _returnvalue)))
    (return)))

(fn `SetupGemMaterialByDamage`
  (params (`Static Mesh Component` :type "StaticMeshComponent Object Reference (by ref)") (DamageType :type "/Game/GeneralLogic/E_DamageType Enum" :default "NewEnumerator0"))
  (`SceneComponent.SetVisibility` `Static Mesh Component` (`|EnumInequality` DamageType "NewEnumerator0") false)
  (switch `/Game/GeneralLogic/E_DamageType` DamageType
    (:`NewEnumerator1`
      (`PrimitiveComponent.SetMaterial` (`local.Static Mesh Component`) 0 (`self.LightningMaterial`)))
    (:`NewEnumerator2`
      (`PrimitiveComponent.SetMaterial` (`local.Static Mesh Component`) 0 (`self.PoisonMaterial`)))
    (:`NewEnumerator4`
      (`PrimitiveComponent.SetMaterial` (`local.Static Mesh Component`) 0 (`self.BloodMaterial`)))
    (:`NewEnumerator5`
      (`PrimitiveComponent.SetMaterial` (`local.Static Mesh Component`) 0 (`self.MagicMaterial`)))))

(fn `SetupGemsInSockets`
  (bind _asbp_player_character (cast `/Game/Player/Logic/BP_PlayerCharacter` (`self.GetOwner`)))
  (bind _returnvalue (`|AddComponentByClass` :`self` (`self.GetOwner`) :`Class` "/Script/Engine.StaticMeshComponent"))
  (bind _output_get (set `self.FastGemMeshComponent` _returnvalue))
  (`StaticMeshComponent.SetStaticMesh` _output_get (`self.FastGemSocketMesh`))
  (bind _weapon (`/Game/Player/Logic/BP_PlayerCharacter.Weapon` _asbp_player_character))
  (`SceneComponent.K2_AttachToComponent` _returnvalue _weapon "FastGemSocket" "SnapToTarget" "SnapToTarget" "SnapToTarget" true)
  (bind _returnvalue_2 (`|AddComponentByClass` :`self` (`self.GetOwner`) :`Class` "/Script/Engine.StaticMeshComponent"))
  (bind _output_get_2 (set `self.HeavyGemMeshComponent` _returnvalue_2))
  (`StaticMeshComponent.SetStaticMesh` _output_get_2 (`self.HeavyGemSocketMesh`))
  (`SceneComponent.K2_AttachToComponent` _returnvalue_2 _weapon "HeavyGemSocket" "SnapToTarget" "SnapToTarget" "SnapToTarget" true)
  (bind _returnvalue_3 (`|AddComponentByClass` :`self` (`self.GetOwner`) :`Class` "/Script/Engine.StaticMeshComponent"))
  (bind _output_get_3 (set `self.MovementGemMeshComponent_1` _returnvalue_3))
  (`StaticMeshComponent.SetStaticMesh` _output_get_3 (`self.MovementGemSocketMesh`))
  (`SceneComponent.K2_AttachToComponent` _returnvalue_3 _weapon "MovementGemSocket_1" "SnapToTarget" "SnapToTarget" "SnapToTarget" true)
  (bind _returnvalue_4 (`|AddComponentByClass` :`self` (`self.GetOwner`) :`Class` "/Script/Engine.StaticMeshComponent"))
  (bind _output_get_4 (set `self.MovementGemMeshComponent_2` _returnvalue_4))
  (`StaticMeshComponent.SetStaticMesh` _output_get_4 (`self.MovementGemSocketMesh`))
  (`SceneComponent.K2_AttachToComponent` _returnvalue_4 _weapon "MovementGemSocket_2" "SnapToTarget" "SnapToTarget" "SnapToTarget" true)
  (for _array_element (`|MakeArray` (`self.FastGemMeshComponent`) (`self.MovementGemMeshComponent_2`) (`self.MovementGemMeshComponent_1`) (`self.HeavyGemMeshComponent`))
    (`PrimitiveComponent.SetCollisionEnabled` _array_element "NoCollision")))

(fn `TryStopCurrentHighlight`
  (bind _highlightedgem (`self.HighlightedGem`)
    (:`then`
      (`/Game/GeneralLogic/Gems/BP_BaseGemPickup.StopHighlight` _highlightedgem)
      (set `self.HighlightedGem` null)
      (`self.OnGemHighlightStop`))
    (:`else`
      _))
  (return))
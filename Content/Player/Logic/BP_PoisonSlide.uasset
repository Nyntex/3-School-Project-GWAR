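; BP_PoisonSlide is a temporary area-of-effect actor that deals periodic damage to enemies on behalf of its owning player.
; Setup stores the damage parameters and player, sizes the sphere, sets the lifespan and starts a looping timer at the given tick rate.
; Each timer tick damages overlapping BP_EnemyBase actors, skipping those too far below the actor, while the owning player remains valid.
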(event `Setup`
  (params (Duration :type "Float (double-precision)") (`Damage per Tick` :type "Float (double-precision)") (`Ticks Per Second` :type "Float (double-precision)") (Radius :type "Float (double-precision)") (Player :type "/Game/Player/Logic/BP_PlayerCharacter Object Reference"))
  (set `self.Duration` Duration)
  (set `self.DamagePerTick` `Damage per Tick`)
  (set `self.TicksPerSecond` `Ticks Per Second`)
  (set `self.DamageRadius` Radius)
  (set `self.OwningPlayer` Player)
  (`SphereComponent.SetSphereRadius` (`self.Sphere`) (`self.DamageRadius`) true)
  (`self.SetLifeSpan` (`self.Duration`))
  (`KismetSystemLibrary.K2_SetTimerDelegate` (delegate `Tick`) (/ 1.0 (`self.TicksPerSecond`)) true))

(event `Tick`
  (bind (_returnvalue_x _returnvalue_y _returnvalue_z) (`KismetMathLibrary.BreakVector` (`self.K2_GetActorLocation`)))
  (`self.OwningPlayer`
    (:`then`
      (for _array_element (`PrimitiveComponent.GetOverlappingActors` (`self.Sphere`) "/Game/Enemies/BaseLogic/BP_EnemyBase.BP_EnemyBase_C")
        (bind (_returnvalue_x_2 _returnvalue_y_2 _returnvalue_z_2) (`KismetMathLibrary.BreakVector` (`self.K2_GetActorLocation` _array_element)))
        (if (>= _returnvalue_z_2 (- _returnvalue_z 50.0))
          (message `/Game/GeneralLogic/BPI_Damageable.ApplyDamage` _array_element (make `/Game/GeneralLogic/S_DamageInfo` (`self.DamageType`) (`self.DamagePerTick`)) (`self.OwningPlayer`)))))
    (:`else`)))

(fn `UserConstructionScript`)
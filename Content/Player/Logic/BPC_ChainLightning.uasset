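; Player chain lightning component that hits a target, then spreads beams and damage to nearby enemies.
; ShootChainLightningAtTarget spawns a Niagara beam, takes damage from player stats and scales down knockback and jump range.
; JumpOverToTargets expands breadth-first in randomly delayed waves, branching to every unchecked enemy in range until jumps or targets run out.
; DamageTarget uses BPI_Damageable, falling back to engine ApplyDamage.
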(event `ShootChainLightningAtTarget`
  (params (StartPosition :type "Vector Structure") (TargetActor :type "Actor Object Reference") (JumpOvers :type Integer) (JumpOverRange :type "Float (double-precision)") (DamageInfo :type "/Game/GeneralLogic/S_DamageInfo Structure"))
  (bind (_damagetype _damageamount _tickinterval _tickamount _knockbackforce _impactlocation) (break `/Game/GeneralLogic/S_DamageInfo` DamageInfo))
  (`self.LightningSystem`
    (:`then`
      (`self.SpawnNewBeam` StartPosition (`Actor.K2_GetActorLocation` TargetActor)) ; The Beam for the original target isn't part of the jump over beams, \ntherefore it stands alone outside of the macro
      (bind _asbp_player_character (cast `/Game/Player/Logic/BP_PlayerCharacter` (`GameplayStatics.GetPlayerCharacter` 0)))
      (bind _s_damageinfo (make `/Game/GeneralLogic/S_DamageInfo` _damagetype (`/Game/Player/Logic/BPC_PlayerStats.ChainLightningDamage` (`/Game/Player/Logic/BP_PlayerCharacter.BPC_PlayerStats` _asbp_player_character)) _tickinterval _tickamount (* _knockbackforce 0.1) _impactlocation))
      (`self.DamageTarget` TargetActor _s_damageinfo)
      (`self.JumpOverToTargets` JumpOvers (* JumpOverRange 0.5) TargetActor _s_damageinfo))
    (:`else`)))

(fn `ClearArrays`
  (`KismetArrayLibrary.Array_Clear` (`self.ActorsToJumpOverFrom`))
  (`KismetArrayLibrary.Array_Clear` (`self.NextToCheck`))
  (`KismetArrayLibrary.Array_Clear` (`self.AlreadyChecked`))
  (return))

(fn `DamageTarget`
  (params (DamageTarget :type "Actor Object Reference") (DamageInfo :type "/Game/GeneralLogic/S_DamageInfo Structure (by ref)"))
  (bind (_damagetype _damageamount _tickinterval _tickamount _knockbackforce _impactlocation) (break `/Game/GeneralLogic/S_DamageInfo` DamageInfo))
  (bind (_damageinfo_damagetype _damageinfo_damageamount) (break `/Game/GeneralLogic/S_DamageInfo` (`local.DamageInfo`)))
  (bind _asbpi_damageable (cast `/Game/GeneralLogic/BPI_Damageable` DamageTarget)
    (:`then`
      (`/Game/GeneralLogic/BPI_Damageable.ApplyDamage` _asbpi_damageable (make `/Game/GeneralLogic/S_DamageInfo` "NewEnumerator1" _damageamount _tickinterval _tickamount _knockbackforce _impactlocation) (`self.GetOwner`)))
    (:`CastFailed`
      (`GameplayStatics.ApplyDamage` (`local.DamageTarget`) _damageinfo_damageamount null (`self.GetOwner`))))
  (return))

(fn `SpawnNewBeam`
  (params (StartPosition :type "Vector Structure") (EndPosition :type "Vector Structure"))
  (bind _returnvalue (`NiagaraFunctionLibrary.SpawnSystemAtLocation` (`self.LightningSystem`) StartPosition))
  (`NiagaraComponent.SetVariablePosition` _returnvalue "Beam Start" StartPosition)
  (`NiagaraComponent.SetVariablePosition` _returnvalue "Beam End" EndPosition))
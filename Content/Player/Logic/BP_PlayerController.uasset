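; Player controller that routes Enhanced Input menu actions to the main menu game mode and tracks whether a gamepad is in use.
; On BeginPlay it caches the main menu game mode, if active, and the game instance.
; Back, confirm and directional actions call the matching game mode functions only when that reference is valid.
; Any key press sets the game instance's GamepadActive flag according to whether it is a gamepad key.
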(event `self.ReceiveBeginPlay`
  (bind _asbp_main_menu_game_mode (cast `/Game/UI/BP_MainMenuGameMode` (`GameplayStatics.GetGameMode`))
    (:`then`
      (set `self.As BP Main Menu Game Mode` _asbp_main_menu_game_mode))
    (:`CastFailed`
      _))
  (bind _asbp_game_instance (cast `/Game/GeneralLogic/BP_GameInstance` (`GameplayStatics.GetGameInstance`)))
  (set `self.As BP Game Instance` _asbp_game_instance))

(event `Key|AnyKey` :consume false
  (params (Key :type "Key Structure"))
  (:`Pressed`
    (set `/Game/GeneralLogic/BP_GameInstance.GamepadActive` (`KismetInputLibrary.Key_IsGamepadKey` Key) (`self.As BP Game Instance`))))

(event `EnhancedInput|/Game/Input/Menu/IA_Menu_Back`
  (params (ActionValue :type Boolean) (ElapsedSeconds :type "Float (double-precision)") (TriggeredSeconds :type "Float (double-precision)") (InputAction :type "InputAction Object Reference" :default "/Game/Input/Menu/IA_Menu_Back.IA_Menu_Back"))
  (:`Started`
    (bind _as_bp_main_menu_game_mode (`self.As BP Main Menu Game Mode`)
      (:`then`
        (`/Game/UI/BP_MainMenuGameMode.MenuBack` _as_bp_main_menu_game_mode))
      (:`else`))))

(event `EnhancedInput|/Game/Input/Menu/IA_Menu_Confirm`
  (params (ActionValue :type Boolean) (ElapsedSeconds :type "Float (double-precision)") (TriggeredSeconds :type "Float (double-precision)") (InputAction :type "InputAction Object Reference" :default "/Game/Input/Menu/IA_Menu_Confirm.IA_Menu_Confirm"))
  (:`Started`
    (bind _as_bp_main_menu_game_mode (`self.As BP Main Menu Game Mode`)
      (:`then`
        (`/Game/UI/BP_MainMenuGameMode.MenuConfirm` _as_bp_main_menu_game_mode))
      (:`else`))))

(event `EnhancedInput|/Game/Input/Menu/IA_Menu_Left`
  (params (ActionValue :type Boolean) (ElapsedSeconds :type "Float (double-precision)") (TriggeredSeconds :type "Float (double-precision)") (InputAction :type "InputAction Object Reference" :default "/Game/Input/Menu/IA_Menu_Left.IA_Menu_Left"))
  (:`Triggered`
    (bind _as_bp_main_menu_game_mode (`self.As BP Main Menu Game Mode`)
      (:`then`
        (`/Game/UI/BP_MainMenuGameMode.MenuLeft` _as_bp_main_menu_game_mode))
      (:`else`))))

(event `EnhancedInput|/Game/Input/Menu/IA_Menu_Right`
  (params (ActionValue :type Boolean) (ElapsedSeconds :type "Float (double-precision)") (TriggeredSeconds :type "Float (double-precision)") (InputAction :type "InputAction Object Reference" :default "/Game/Input/Menu/IA_Menu_Right.IA_Menu_Right"))
  (:`Triggered`
    (bind _as_bp_main_menu_game_mode (`self.As BP Main Menu Game Mode`)
      (:`then`
        (`/Game/UI/BP_MainMenuGameMode.MenuRight` _as_bp_main_menu_game_mode))
      (:`else`))))

(event `EnhancedInput|/Game/Input/Menu/IA_Menu_Up`
  (params (ActionValue :type Boolean) (ElapsedSeconds :type "Float (double-precision)") (TriggeredSeconds :type "Float (double-precision)") (InputAction :type "InputAction Object Reference" :default "/Game/Input/Menu/IA_Menu_Up.IA_Menu_Up"))
  (:`Started`
    (bind _as_bp_main_menu_game_mode (`self.As BP Main Menu Game Mode`)
      (:`then`
        (`/Game/UI/BP_MainMenuGameMode.MenuUp` _as_bp_main_menu_game_mode))
      (:`else`))))

(event `EnhancedInput|/Game/Input/Menu/IA_Menu_Down`
  (params (ActionValue :type Boolean) (ElapsedSeconds :type "Float (double-precision)") (TriggeredSeconds :type "Float (double-precision)") (InputAction :type "InputAction Object Reference" :default "/Game/Input/Menu/IA_Menu_Down.IA_Menu_Down"))
  (:`Started`
    (bind _as_bp_main_menu_game_mode (`self.As BP Main Menu Game Mode`)
      (:`then`
        (`/Game/UI/BP_MainMenuGameMode.MenuDown` _as_bp_main_menu_game_mode))
      (:`else`))))

(fn `UserConstructionScript`)
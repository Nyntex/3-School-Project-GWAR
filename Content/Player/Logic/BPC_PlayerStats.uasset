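; BPC_PlayerStats is a player component that tracks health and damage reduction.
; ReduceHealth scales damage by the total reduction, while AddHealth clamps to max; both report the health fraction, and ReduceHealth signals depletion at zero or below.
; Blood Shield adds timed reduction through the clamped adjustment event, and reapplying it removes the active bonus and restarts the timer instead of stacking.
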(event `ReduceHealth`
  (params (Amount :type "Float (double-precision)"))
  (bind _output_get (set `self.CurrHealth` (- (`self.CurrHealth`) (- Amount (* Amount (`self.TotalDamageReduction`))))))
  (`self.HealthChanged` (/ _output_get (`self.MaxHealth`)))
  (if (<= _output_get 0.0)
    (`self.HealthDepleted`)))

(event `AddHealth`
  (params (Amount :type "Float (double-precision)"))
  (bind _output_get (set `self.CurrHealth` (`KismetMathLibrary.FClamp` (+ (`self.CurrHealth`) Amount) 0.0 (`self.MaxHealth`))))
  (`self.HealthChanged` (/ _output_get (`self.MaxHealth`))))

(event `AdjustDamageReduction`
  (params (Amount :type "Float (double-precision)"))
  (set `self.TotalDamageReduction` (`KismetMathLibrary.FClamp` (+ Amount (`self.TotalDamageReduction`)))))

(event `ApplyBloodShield`
  (bind _bloodshieldtimer (`self.BloodShieldTimer`))
  (if (`KismetSystemLibrary.K2_IsValidTimerHandle` _bloodshieldtimer)
    (`KismetSystemLibrary.K2_ClearAndInvalidateTimerHandle` _bloodshieldtimer)
    (`self.RemoveBloodShield`))
  (bind _returnvalue (`KismetSystemLibrary.K2_SetTimerDelegate` (delegate `RemoveBloodShield`) (`self.BloodShieldDuration`)))
  (set `self.BloodShieldTimer` _returnvalue)
  (`self.AdjustDamageReduction` (`self.BloodShieldReductionValue`)))

(event `RemoveBloodShield`
  (`self.AdjustDamageReduction` (* (`self.BloodShieldReductionValue`) -1.0)))
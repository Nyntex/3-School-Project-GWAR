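; Enemy component for kicked behaviour that can kill its BP_EnemyBase owner on impact.
; Shortly after BeginPlay it binds to the owner's actor hit event and reacts once to a non-Pawn hit.
; Below half health, the enemy gets splat effects, dies and is destroyed; otherwise the component removes itself after a short delay.
; The kill-time check is never called, and the triggerable activation is disconnected, marked as possibly deprecated.
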(event `self.ReceiveBeginPlay`
  (set `self.StartTime` (`KismetSystemLibrary.GetGameTimeInSeconds`))
  (bind _asbp_enemy_base (cast `/Game/Enemies/BaseLogic/BP_EnemyBase` (`self.GetOwner`)))
  (bind _output_get (set `self.Owner` _asbp_enemy_base))
  (`KismetSystemLibrary.Delay` 0.1)
  (add `Actor.OnActorHit` _output_get (delegate `OwnerHit`)))

(event `OwnerHit`
  (params (SelfActor :type "Actor Object Reference") (OtherActor :type "Actor Object Reference") (NormalImpulse :type "Vector Structure") (Hit :type "HitResult Structure (by ref)"))
  (bind _owner (`self.Owner`))
  (cast `Pawn` OtherActor
    (:`CastFailed`
      (`/Engine/EditorBlueprintResources/StandardMacros.DoOnce` false
        (:`Completed`
          (if (`self.IsHealthThresholdReched`)
            (`self.PlayEffects` (`.ImpactPoint` (`GameplayStatics.BreakHitResult` Hit)))
            (`/Game/Enemies/BaseLogic/BP_EnemyBase.Die` _owner _owner)
            (`Actor.K2_DestroyActor` _owner)
            (else
              (`self.EndBehaviour`))))))))

(fn `IsHealthThresholdReched`
  (returns (ReturnValue :type Boolean))
  (bind _owner (`self.Owner`))
  (return (< (`EnemyBase.currentHealth` _owner) (* (`EnemyBase.maxHealth` _owner) 0.5))))

(fn `IsKillTimeReached`
  (returns (ReturnValue :type Boolean))
  (return (> (- (`KismetSystemLibrary.GetGameTimeInSeconds`) (`self.StartTime`)) (`self.KillTime`))))

(fn `PlayEffects`
  (params (Location :type "Vector Structure"))
  (`NiagaraFunctionLibrary.SpawnSystemAtLocation` "/Game/Enemies/VFX/Hit_FX/NS_Enemy_Hit_Neutral.NS_Enemy_Hit_Neutral" Location (struct) (5.0 5.0 5.0))
  (`GameplayStatics.PlaySoundAtLocation` "/Game/Audio/SFX/MetaSounds/MS_EnemySplat.MS_EnemySplat" Location (struct) 1.0 1.0 0.0 null null null null))

(fn `TryActivateTriggerable`
  (params (HitActor :type "Actor Object Reference"))
  (if (`KismetSystemLibrary.DoesImplementInterface` HitActor "/Game/GeneralLogic/BPI_Triggerable.BPI_Triggerable_C")
    (bind _asibp_triggerable (cast `/Game/GeneralLogic/BPI_Triggerable` HitActor))
    (`/Game/GeneralLogic/BPI_Triggerable.Trigger` _asibp_triggerable))
  (return))
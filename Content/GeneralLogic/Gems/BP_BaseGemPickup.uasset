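; Base actor for a gem pickup that can be highlighted and collected, carrying a gem type and slot type.
; On BeginPlay it sets the gem material by type and copies the mesh onto an overlay component that uses a fixed highlight material.
; Highlight and StopHighlight toggle that overlay and an interact widget.
; Pickup broadcasts OnPickup, destroys the actor and returns both types; the widget's camera-facing rotation logic is disconnected.
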(event `self.ReceiveBeginPlay`
  (`self.ReloadMaterial`)
  (`StaticMeshComponent.SetStaticMesh` (`self.GemHighlighted`) (`StaticMeshComponent.StaticMesh` (`self.Gem`))))

(event `self.ReceiveTick`
  (params (DeltaSeconds :type "Float (single-precision)")))

(event `ReloadMaterial`
  (bind _materials (`self.Materials`))
  (`/Engine/EditorBlueprintResources/StandardMacros.IsValid` (`StaticMeshComponent.StaticMesh` (`self.Gem`))
    (:`Is Valid`
      (`PrimitiveComponent.SetMaterial` (`self.Gem`) 0 (`|GetArrayItem` _materials (`KismetMathLibrary.Conv_ByteToInt` (`self.GemType`))))
      (`PrimitiveComponent.SetMaterial` (`self.GemHighlighted`) 0 (`|GetArrayItem` _materials 5)))))

(fn `Highlight`
  (if (not (`self.Highlighted`))
    (set `self.Highlighted` true)
    (`SceneComponent.SetVisibility` (`self.GemHighlighted`) true false)
    (`SceneComponent.SetVisibility` (`self.InteractWidget`) true false)))

(fn `Pickup`
  (returns (GemSlotType :type "/Game/Player/Logic/E_GemSlot Enum") (GemType :type "/Game/GeneralLogic/E_DamageType Enum"))
  (`self.OnPickup` (`self.GemSlotType`) (`self.GemType`))
  (`self.K2_DestroyActor`)
  (return (`self.GemSlotType`) (`self.GemType`)))

(fn `StopHighlight`
  (if (`self.Highlighted`)
    (set `self.Highlighted` false)
    (`self.ReloadMaterial`)
    (`SceneComponent.SetVisibility` (`self.GemHighlighted`) false false)
    (`SceneComponent.SetVisibility` (`self.InteractWidget`) false false)))

(fn `UserConstructionScript`)
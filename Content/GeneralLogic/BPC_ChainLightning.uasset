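; Actor component that fires chain lightning from a start actor to a target, then spreads it to nearby actors over a set number of jumps.
; Each jump sphere-overlaps pawns and world dynamic objects around the current wave of actors, and every actor found seeds the next wave, so chains branch breadth-first.
; Each damageable actor not already in the LightningBolts map gets a BPC_Beam component carrying endpoints, causer and damage.
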(event `ShootChainAtTarget`
  (params (TargetActor :type "Actor Object Reference") (StartActor :type "Actor Object Reference") (Damage :type "Float (double-precision)") (JumpOvers :type Integer))
  (bind _nextactorstocheck (`self.NextActorsToCheck`))
  (`self.SummonLightningBeam` TargetActor (`self.GetOwner`) StartActor Damage)
  (set `self.currentActorsToCheck` (`|MakeArray` TargetActor))
  (for _ (range JumpOvers)
    (`|ExecutionSequence`
      (:`then_0`
        (for _array_element (`self.currentActorsToCheck`)
          (bind _outactors (`KismetSystemLibrary.SphereOverlapActors` (`Actor.K2_GetActorLocation` _array_element) (`self.Range`) (`|MakeArray` "ObjectTypeQuery3" "ObjectTypeQuery2" :!type "EObjectTypeQuery Enum") null (`self.currentActorsToCheck`)))
          (for _array_element_2 _outactors
            (`KismetArrayLibrary.Array_Add` (`self.NextActorsToCheck`) _array_element_2)
            (`self.SummonLightningBeam` _array_element_2 _array_element _array_element Damage))))
      (:`then_1`
        (`KismetArrayLibrary.Array_Clear` (`self.currentActorsToCheck`))
        (set `self.currentActorsToCheck` _nextactorstocheck)
        (`KismetArrayLibrary.Array_Clear` _nextactorstocheck)))))

(fn `SummonLightningBeam`
  (params (EndActor :type "Actor Object Reference") (BeamOwner :type "Actor Object Reference") (StartActor :type "Actor Object Reference") (Damage :type "Float (double-precision)"))
  (bind _endactor (`local.EndActor`))
  (if (`Actor.bCanBeDamaged` EndActor)
    (if (not (`.ReturnValue` (`BlueprintMapLibrary.Map_Find` (`self.LightningBolts`) EndActor)))
      (bind _returnvalue (`|AddComponentByClass` (`local.BeamOwner`) "/Game/GeneralLogic/BPC_Beam.BPC_Beam_C"))
      (`BlueprintMapLibrary.Map_Add` (`self.LightningBolts`) _endactor _returnvalue)
      (set `/Game/GeneralLogic/BPC_Beam.End` _endactor _returnvalue)
      (set `/Game/GeneralLogic/BPC_Beam.Start` (`local.StartActor`) _returnvalue)
      (set `/Game/GeneralLogic/BPC_Beam.Causer` (`self.GetOwner`) _returnvalue)
      (set `/Game/GeneralLogic/BPC_Beam.Damage` (`local.Damage`) _returnvalue))))
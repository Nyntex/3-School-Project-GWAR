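; BP_DefaultGameMode is the default game mode, handling level transitions behind a loading screen.
; The WBP_Loading widget is created if needed and referenced on BP_GameInstance; BeginPlay plays its fade-out, hides it after a delay and unpauses the game.
; LoadLevel shows the screen with the fade reversed at higher speed, async-loads a primary asset chosen by level name, then opens that level after a short delay.
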(event `self.ReceiveBeginPlay`
  (bind _asbp_game_instance (cast `/Game/GeneralLogic/BP_GameInstance` (`GameplayStatics.GetGameInstance`)))
  (bind _output_get (set `self.As BP Game Instance` _asbp_game_instance))
  (`self.TryCreateLoadingScreen` _output_get)
  (bind _loadingscreen (`/Game/GeneralLogic/BP_GameInstance.LoadingScreen` _output_get))
  (`UserWidget.AddToPlayerScreen` _loadingscreen 100)
  (`Widget.SetVisibility` _loadingscreen "Visible")
  (`UserWidget.PlayAnimation` _loadingscreen (`/Game/UI/OtherWidgets/WBP_Loading.FadeOut` _loadingscreen) 0.0 1 "Forward" 1.0 false)
  (`KismetSystemLibrary.Delay` 3.0)
  (`Widget.SetVisibility` _loadingscreen "Hidden")
  (`GameplayStatics.SetGamePaused` false))

(event `LoadLevel`
  (params (Level :type "World Soft Object Reference") (LevelName :type Name))
  (bind _loadingscreen (`/Game/GeneralLogic/BP_GameInstance.LoadingScreen` (`self.As BP Game Instance`)))
  (`Widget.SetVisibility` _loadingscreen "Visible")
  (`UserWidget.PlayAnimation` _loadingscreen (`/Game/UI/OtherWidgets/WBP_Loading.FadeOut` _loadingscreen) 0.0 1 "Reverse" 5.0 false)
  (switch `name` LevelName
    (:`Default`
      (`AsyncActionLoadPrimaryAsset.AsyncLoadPrimaryAsset` "Map:/Game/Maps/Level_Cave_V1"
        (:`Completed`
          _)))
    (:`Level_Cave_V1`
      (`AsyncActionLoadPrimaryAsset.AsyncLoadPrimaryAsset` "Map:/Game/Maps/Level_Cave_V1"
        (:`Completed`
          _)))
    (:`Level_Daniel`
      (`AsyncActionLoadPrimaryAsset.AsyncLoadPrimaryAsset` "Map:/Game/Maps/Level_Daniel"
        (:`Completed`
          _)))
    (:`Level_Anni`
      (`AsyncActionLoadPrimaryAsset.AsyncLoadPrimaryAsset` "Map:/Game/Maps/Level_Anni"
        (:`Completed`
          _)))
    (:`Level_K3`
      (`AsyncActionLoadPrimaryAsset.AsyncLoadPrimaryAsset` "Map:/Game/Maps/Level_K3"
        (:`Completed`
          _))))
  (`KismetSystemLibrary.Delay` 0.2)
  (`GameplayStatics.OpenLevel` LevelName))

(fn `TryCreateLoadingScreen`
  (params (GameInstance :type "/Game/GeneralLogic/BP_GameInstance Object Reference"))
  (`/Engine/EditorBlueprintResources/StandardMacros.IsValid` (`/Game/GeneralLogic/BP_GameInstance.LoadingScreen` GameInstance)
    (:`Is Valid`
      _)
    (:`Is Not Valid`
      (bind _returnvalue (`|CreateWidget` "/Game/UI/OtherWidgets/WBP_Loading.WBP_Loading_C" (`GameplayStatics.GetPlayerController` 0)))
      (`UserWidget.AddToViewport` _returnvalue 0)
      (set `/Game/GeneralLogic/BP_GameInstance.LoadingScreen` _returnvalue GameInstance)))
  (return))

(fn `UserConstructionScript`)
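; Actor component that draws a temporary Niagara beam between Start and End actors and damages its owner.
; BeginPlay spawns the system, applies one damage hit through BPI_Damageable, then destroys the component after Duration.
; Tick feeds both actor locations into the beam's endpoint variables; its visibility trace result does not affect the endpoint.
; EndPlay removes the spawned Niagara system.
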(event `self.ReceiveBeginPlay`
  (bind _niagarasystem (`self.NiagaraSystem`)
    (:`then`
      (bind _returnvalue (`NiagaraFunctionLibrary.SpawnSystemAtLocation` _niagarasystem (`Actor.K2_GetActorLocation` (`self.GetOwner`))))
      (set `self.SpawnedSystem` _returnvalue)
      (bind _asbpi_damageable (cast `/Game/GeneralLogic/BPI_Damageable` (`self.GetOwner`))
        (:`then`
          (`/Game/GeneralLogic/BPI_Damageable.ApplyDamage` _asbpi_damageable (make `/Game/GeneralLogic/S_DamageInfo` "NewEnumerator1" (`self.Damage`)) (`self.Causer`)))
        (:`CastFailed`
          _))
      (`KismetSystemLibrary.Delay` (`self.Duration`)))
    (:`else`
      _))
  (`self.K2_DestroyComponent`))

(event `Reposition`
  (`NiagaraComponent.SetVariableVec3` (`self.SpawnedSystem`) "Beam Start" (`Actor.K2_GetActorLocation` (`self.Start`)))
  (bind _outhit (`KismetSystemLibrary.LineTraceSingle` (`Actor.K2_GetActorLocation` (`self.Start`)) (`Actor.K2_GetActorLocation` (`self.End`)) "TraceTypeQuery1"))
  (if (`GameplayStatics.BreakHitResult` _outhit)
    _
    (else
      _))
  (`NiagaraComponent.SetVariableVec3` (`self.SpawnedSystem`) "Beam End" (`Actor.K2_GetActorLocation` (`self.End`))))

(event `self.ReceiveEndPlay`
  (params (EndPlayReason :type "EEndPlayReason Enum" :default "Destroyed"))
  (`self.K2_DestroyComponent` (`self.SpawnedSystem`)))

(event `self.ReceiveTick`
  (params (DeltaSeconds :type "Float (single-precision)"))
  (`self.Reposition`))

(fn `IsValid`
  (returns (IsValid :type Boolean))
  (`self.Start`
    (:`then`
      (`self.End`
        (:`then`
          (return true))
        (:`else`
          _)))
    (:`else`
      _))
  (return false))